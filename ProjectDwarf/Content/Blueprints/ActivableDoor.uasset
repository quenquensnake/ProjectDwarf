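; Activable door that slides open once all of its linked interruptors and switches are toggled on.
; The opening trigger checks both arrays, then plays a timeline that lerps the door's relative location from its start to that start plus a configurable offset.
; The closing trigger reverses the timeline unless MustToggle is set, without rechecking switch states.
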(event `self.ReceiveBeginPlay`
  (bind _output_get (set `self.Door_Starting_Location` (`SceneComponent.RelativeLocation` (`self.Door`))))
  (set `self.Door_End_Location` (+ _output_get (`self.Door_Offset`))))

(event `Door_Trigger_Opening`
  ;[1 1 1] Check if each interruptors is toggled
  (set `self.All_Interruptor_Activated` true)
  (for _array_element (`self.tab_interrupt`)
    (if (not (`/Game/Blueprints/Pressure_plate_BP.Is_Toggled_On` _array_element))
      (set `self.All_Interruptor_Activated` false)))
  (for _array_element_2 (`self.tab_switches`)
    (if (not (`/Game/Blueprints/Interaction/InteractionSwitch_BP.Is_Toggled_On` _array_element_2))
      (set `self.All_Interruptor_Activated` false)))
  (if (`self.All_Interruptor_Activated`)
    ;[1 1 1] Move Door
    (bind (_direction _moving) (`Timeline|Door_Opening` :!label _label)
      (:`Update`
        (`SceneComponent.K2_SetRelativeLocation` (`self.Door`) (`KismetMathLibrary.VLerp` (`self.Door_Starting_Location`) (`self.Door_End_Location`) _moving) false false)))))

(event `Door_Trigger_Closing`
  ;[1 1 1] Close the door if configured in No Toggle mode
  (if (not (`self.Must_Toggle`))
    (goto _label :!via `Reverse`)))

(fn `NewFunction_0`)

(fn `UserConstructionScript`)