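; CameraRotator is a trigger box that smoothly turns the game mode's camera to a set yaw when the player enters it.
; On overlap it cancels any rotation running on other CameraRotators, then starts a looping timer at the current frame's delta time.
; Each tick lerps yaw toward AddZAngle, an absolute target despite its name, by shortest path, stopping once the rounded 360-converted yaw matches.
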(event `self.Box.OnComponentBeginOverlap`
  (params (OverlappedComponent :type "PrimitiveComponent Object Reference") (OtherActor :type "Actor Object Reference") (OtherComp :type "PrimitiveComponent Object Reference") (OtherBodyIndex :type Integer) (bFromSweep :type Boolean) (SweepResult :type "HitResult Structure (by ref)"))
  (if (not (`self.IsRotating?`))
    (if (== (`GameplayStatics.GetObjectClass` OtherActor) "/Game/Blueprints/Player_BP.Player_BP_C")
      ;[1 0 0] Reset other current rotations
      (bind _outactors (`GameplayStatics.GetAllActorsOfClass` "CameraRotator_C"))
      (for _array_element _outactors
        (if (`/Game/Blueprints/CameraRotator.IsRotating?` _array_element)
          (`KismetSystemLibrary.K2_ClearAndInvalidateTimerHandle` (`/Game/Blueprints/CameraRotator.TimerHandle` _array_element))
          (set `/Game/Blueprints/CameraRotator.IsRotating?` false _array_element)))
      ;[1 1 0] Loop creation for rotation
      (bind _asgame_mode_bp (cast `/Game/Blueprints/GameMode_BP` (`GameplayStatics.GetGameMode`)))
      (set `self.IsRotating?` true)
      (bind _returnvalue (`KismetSystemLibrary.K2_SetTimer` null "RotateCam" (`GameplayStatics.GetWorldDeltaSeconds`) true)) ; Boucle pour que la rotation en lerp se fasse
      (bind _output_get (set `self.TimerHandle` _returnvalue)))))

(event `RotateCam`
  (bind _addzangle (`self.AddZAngle`))
  ;[0.01 1 0] Rotation
  (bind _camerabp (`/Game/Blueprints/GameMode_BP.CameraBP` (stale `self.Box.OnComponentBeginOverlap` _asgame_mode_bp)))
  (bind _returnvalue (`self.K2_GetActorRotation` _camerabp))
  (`self.K2_SetActorRotation` _camerabp (`KismetMathLibrary.RLerp` _returnvalue (`KismetMathLibrary.MakeRotator` (.roll _returnvalue) (.pitch _returnvalue) _addzangle) (* (`GameplayStatics.GetWorldDeltaSeconds`) (`self.SpeedRotation`)) true) false)
  (bind _new_angle (`/Game/Blueprints/SuperLib.Angle360Convert` (.yaw _returnvalue)))
  (if (== (`KismetMathLibrary.Round` _new_angle) (`KismetMathLibrary.Round` _addzangle))
    (`KismetSystemLibrary.K2_ClearAndInvalidateTimerHandle` (stale `self.Box.OnComponentBeginOverlap` _output_get))
    (set `self.IsRotating?` false)))

(fn `UserConstructionScript`)