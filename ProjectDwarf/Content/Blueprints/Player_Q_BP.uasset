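; Player Blueprint with control-yaw-relative movement and an early grappling hook that attaches a visible cable to the world.
; The grapnel input traces forward and slightly down from the mesh on the Visibility channel, with debug drawing.
; On a hit, it spawns an anchor actor there, attaches the cable to it and sets the cable length to that distance.
; The cable starts hidden; no pull or release logic exists.
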(event `InputAxis|MoveForward`
  (params (AxisValue :type "Float (single-precision)"))
  ;[1 1 1] Mouvements
  (`self.AddMovementInput` (`KismetMathLibrary.GetForwardVector` (`KismetMathLibrary.MakeRotator` 0.0 0.0 (.yaw (`self.GetControlRotation`)))) AxisValue))

(event `InputAxis|MoveRight`
  (params (AxisValue :type "Float (single-precision)"))
  ;[1 1 1] Mouvements
  (`self.AddMovementInput` (`KismetMathLibrary.GetRightVector` (`KismetMathLibrary.MakeRotator` 0.0 0.0 (.yaw (`self.GetControlRotation`)))) AxisValue))

(event `InputAction|grapnel`
  (params (Key :type "Key Structure" :default "AnyKey"))
  (bind _cable (`self.Cable`))
  (bind _returnvalue (`SceneComponent.K2_GetComponentLocation` (`self.Mesh`)))
  (:`Pressed`
    (bind (_outhit _returnvalue_2) (`KismetSystemLibrary.LineTraceSingle` :`Start` _returnvalue :`End` (+ _returnvalue (+ (* (`SceneComponent.GetForwardVector` (`self.Mesh`)) 1000.0) (0.0 0.0 -150.0))) :`TraceChannel` "TraceTypeQuery1" :`bTraceComplex` true :`DrawDebugType` "ForDuration" :`TraceColor` (struct :`R` 0.031642 :`G` 0.060844 :`B` 1.0 :`A` 1.0)))
    (if _returnvalue_2
      (`KismetSystemLibrary.PrintString` "MDR")
      (`SceneComponent.SetVisibility` (`self.Cable`) true false)
      (bind _returnvalue_3 (`|SpawnActorFromClass` "/Game/Blueprints/CableAttachEnd.CableAttachEnd_C" (`KismetMathLibrary.Conv_VectorToTransform` (`.Location` (`GameplayStatics.BreakHitResult` _outhit))) "Undefined" "OverrideRootScale"))
      (bind _output_get (set `self.CableAttachEnd` _returnvalue_3))
      (`CableComponent.SetAttachEndTo` _cable _output_get "None" "None")
      (set `CableComponent.CableLength` (`KismetMathLibrary.VSize` (- (`self.K2_GetActorLocation` (`self.CableAttachEnd`)) (`SceneComponent.K2_GetComponentLocation` (`self.Mesh`)))) _cable))))

(event `self.ReceiveBeginPlay`
  (`SceneComponent.SetVisibility` (`self.Cable`) false false))

(fn `UserConstructionScript`)