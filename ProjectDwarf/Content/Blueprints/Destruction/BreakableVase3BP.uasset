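; BreakableVase3BP is a destructible vase that shatters after taking enough hits.
; Each damage event decrements Health, and at zero a DoOnce enables physics simulation on the Destructible component.
; If the damage causer is an Axe_BP, it then applies radius damage with impulse at the axe's ImpactPoint, so the break originates where the axe struck.
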(event `self.ReceiveAnyDamage`
  (params (Damage :type "Float (single-precision)") (DamageType :type "DamageType Object Reference") (InstigatedBy :type "Controller Object Reference") (DamageCauser :type "Actor Object Reference"))
  (bind _health (`self.Health`))
  ;[1 1 1] Getting damaged
  (`/Engine/EditorBlueprintResources/StandardMacros.DecrementInt` _health
    (:`  `
      (if (<= _health 0)
        (`/Engine/EditorBlueprintResources/StandardMacros.DoOnce` false
          (:`Completed`
            (`PrimitiveComponent.SetSimulatePhysics` (`self.Destructible`) true)
            (bind _asaxe_bp (cast `/Game/Blueprints/Axe_BP` DamageCauser))
            (`DestructibleComponent.ApplyRadiusDamage` (`self.Destructible`) 80.0 (`/Game/Blueprints/Axe_BP.ImpactPoint` _asaxe_bp) 40.0 3000.0 true)))))))

(fn `UserConstructionScript`)