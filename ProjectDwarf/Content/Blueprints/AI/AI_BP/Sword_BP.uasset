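; Sword weapon Blueprint for the AI character that deals melee damage through traces rather than its own collision.
; Attack and AttackWithJump each sphere-trace on the Camera channel from the AI's location forward by WeaponRange, ignoring the AI and its helmet.
; Every hit spawns an impact particle and receives damage, with the jump attack dealing double.
; Explosion sound calls are present but unconnected.
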(event `Attack`
  (bind _ai_bp_ref (`self.AI_BP_Ref`))
  (bind _returnvalue (`self.K2_GetActorLocation` _ai_bp_ref))
  (bind (_outhits _returnvalue_2) (`KismetSystemLibrary.SphereTraceMulti` _returnvalue (+ _returnvalue (* (`self.GetActorForwardVector` _ai_bp_ref) (`self.WeaponRange`))) 25.0 "TraceTypeQuery2" false (`|MakeArray` _ai_bp_ref (`self.Helmet_BP_Ref`) null :!type "Actor Object Reference")))
  (if _returnvalue_2
    (for _array_element _outhits
      (bind (_bblockinghit _binitialoverlap _time _location _impactpoint _normal _impactnormal _physmat _hitactor) (`GameplayStatics.BreakHitResult` _array_element))
      (set `self.ImpactPoint` _impactpoint)
      (`GameplayStatics.SpawnEmitterAtLocation` "/Game/Particles/P_ImpactAxe.P_ImpactAxe" _location)
      (`GameplayStatics.ApplyDamage` _hitactor 1.0 null self))))

(event `AttackWithJump`
  (bind _ai_bp_ref (`self.AI_BP_Ref`))
  (bind _returnvalue (`self.K2_GetActorLocation` _ai_bp_ref))
  (bind (_outhits _returnvalue_2) (`KismetSystemLibrary.SphereTraceMulti` _returnvalue (+ _returnvalue (* (`self.GetActorForwardVector` _ai_bp_ref) (`self.WeaponRange`))) 25.0 "TraceTypeQuery2" false (`|MakeArray` _ai_bp_ref (`self.Helmet_BP_Ref`) :!type "Actor Object Reference")))
  (if _returnvalue_2
    (for _array_element _outhits
      (bind (_bblockinghit _binitialoverlap _time _location _impactpoint _normal _impactnormal _physmat _hitactor) (`GameplayStatics.BreakHitResult` _array_element))
      (set `self.ImpactPoint` _impactpoint)
      (`GameplayStatics.SpawnEmitterAtLocation` "/Game/Particles/P_ImpactAxe.P_ImpactAxe" _location)
      (`GameplayStatics.ApplyDamage` _hitactor 2.0 null self))))

(fn `UserConstructionScript`)