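; AI knight enemy character that carries a sword and a separate helmet actor, spawning and attaching both on BeginPlay.
; Tick syncs helmet state to the Blackboard and copies attack, stun and helmet-replacement flags back into Blueprint variables.
; With the helmet on, damage builds toward a timed stun relayed to the helmet.
; With it off, damage drains Life, ending in ragdoll and delayed destruction of all three actors.
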(event `self.ReceiveBeginPlay`
  (bind (_returnvalue_location _returnvalue_rotation _returnvalue_scale) (`KismetMathLibrary.BreakTransform` (`self.GetTransform`)))
  (bind _returnvalue (`|SpawnActorFromClass` "/Game/Blueprints/AI/AI_BP/Sword_BP.Sword_BP_C" (`KismetMathLibrary.MakeTransform` _returnvalue_location (struct) _returnvalue_scale) "AlwaysSpawn" "OverrideRootScale"))
  (set `/Game/Blueprints/AI/AI_BP/Sword_BP.AI_BP_Ref` self _returnvalue)
  (bind _output_get (set `self.SwordRef` _returnvalue))
  (`PrimitiveComponent.SetSimulatePhysics` (`/Game/Blueprints/AI/AI_BP/Sword_BP.StaticMesh` _returnvalue) false)
  (`self.K2_AttachToComponent` _returnvalue (`self.Mesh`) "KnightSwordSocket" "SnapToTarget" "SnapToTarget" "SnapToTarget" true)
  (bind _returnvalue_2 (`|SpawnActorFromClass` "/Game/Blueprints/Interaction/Interactibles/Stuff/KnightHelmet_BP.KnightHelmet_BP_C" (`KismetMathLibrary.MakeTransform` _returnvalue_location (struct :`Yaw` -90.0) _returnvalue_scale) "AlwaysSpawn" "OverrideRootScale"))
  (set `/Game/Blueprints/AI/AI_BP/Sword_BP.Helmet_BP_Ref` _returnvalue_2 _output_get)
  (set `self.HelmetRef` _returnvalue_2)
  (`/Game/Blueprints/Interaction/Interactibles/Stuff/KnightHelmet_BP.AttachToKnight` _returnvalue_2 self)
  (`BlackboardComponent.SetValueAsBool` (`AIBlueprintHelperLibrary.GetBlackboard` null) "HeadOnKnight" (`self.HeadOnKnightAI`))
  (`BlackboardComponent.SetValueAsObject` (`AIBlueprintHelperLibrary.GetBlackboard` null) "HelmetActor" _returnvalue_2)
  (`BlackboardComponent.SetValueAsFloat` (`AIBlueprintHelperLibrary.GetBlackboard` null) "Life" (`self.Life`)))

(event `Run`
  (set `CharacterMovementComponent.MaxWalkSpeed` 300.0 (`self.CharacterMovement`)))

(event `self.CapsuleComponent.OnComponentBeginOverlap`
  (params (OverlappedComponent :type "PrimitiveComponent Object Reference") (OtherActor :type "Actor Object Reference") (OtherComp :type "PrimitiveComponent Object Reference") (OtherBodyIndex :type Integer) (bFromSweep :type Boolean) (SweepResult :type "HitResult Structure (by ref)"))
  ;[1 1 1] Getting damaged
)

(event `self.ReceiveTick`
  (params (DeltaSeconds :type "Float (single-precision)"))
  (`BlackboardComponent.SetValueAsBool` (`AIBlueprintHelperLibrary.GetBlackboard` null) "HeadOnKnight" (`self.HeadOnKnightAI`))
  (set `self.AttacksAI` (`BlackboardComponent.GetValueAsBool` (`AIBlueprintHelperLibrary.GetBlackboard` null) "Attacks"))
  (set `self.AttackWithJumpAI` (`BlackboardComponent.GetValueAsBool` (`AIBlueprintHelperLibrary.GetBlackboard` null) "AttackWithJump"))
  (set `self.AttackSimpleAI` (`BlackboardComponent.GetValueAsBool` (`AIBlueprintHelperLibrary.GetBlackboard` null) "AttackSimple"))
  (set `self.WalkForAttackPlayer` (`BlackboardComponent.GetValueAsBool` (`AIBlueprintHelperLibrary.GetBlackboard` null) "WalkForAttackPlayer"))
  (set `self.IsStunned` (`BlackboardComponent.GetValueAsBool` (`AIBlueprintHelperLibrary.GetBlackboard` null) "IsStunned"))
  (bind _output_get (set `self.PutBackHelmetAI` (`BlackboardComponent.GetValueAsBool` (`AIBlueprintHelperLibrary.GetBlackboard` null) "PutBackHelmet")))
  (if _output_get
    (`KismetSystemLibrary.Delay` 4.0)
    (`BlackboardComponent.SetValueAsBool` (`AIBlueprintHelperLibrary.GetBlackboard` null) "PutBackHelmet" false)))

(event `self.ReceiveAnyDamage`
  (params (Damage :type "Float (single-precision)") (DamageType :type "DamageType Object Reference") (InstigatedBy :type "Controller Object Reference") (DamageCauser :type "Actor Object Reference"))
  (bind _mesh (`self.Mesh`))
  ;[1 1 1] Apply Damage to a Player
  (if (not (`self.HeadOnKnightAI`))
    (bind _output_get (set `self.Life` (- (`self.Life`) Damage) :!label _label))
    (`BlackboardComponent.SetValueAsFloat` (`AIBlueprintHelperLibrary.GetBlackboard` null) "Life" _output_get)
    (if (<= (`self.Life`) 0.0)
      (`PrimitiveComponent.SetCollisionEnabled` _mesh "QueryAndPhysics")
      (`SkeletalMeshComponent.SetAllBodiesSimulatePhysics` _mesh true)
      (`KismetSystemLibrary.Delay` 5.0)
      (`self.K2_DestroyActor` (`self.SwordRef`))
      (`self.K2_DestroyActor` (`self.HelmetRef`))
      (`self.K2_DestroyActor`))
    (elif (`BlackboardComponent.GetValueAsBool` (`AIBlueprintHelperLibrary.GetBlackboard` null) "IsStunned")
      (if (not (`self.HeadOnKnightAI`))
        (goto _label))
      (else
        (set `self.StunnedHit` (- (`self.StunnedHit`) Damage))
        (if (<= (`self.StunnedHit`) 0.0)
          (`BlackboardComponent.SetValueAsBool` (`AIBlueprintHelperLibrary.GetBlackboard` null) "IsStunned" true)
          (`/Game/Blueprints/Interaction/Interactibles/Stuff/KnightHelmet_BP.Stun` (`self.HelmetRef`))
          (`KismetSystemLibrary.Delay` 5.0)
          (`BlackboardComponent.SetValueAsBool` (`AIBlueprintHelperLibrary.GetBlackboard` null) "IsStunned" false)
          (set `self.StunnedHit` 3.0)
          (`/Game/Blueprints/Interaction/Interactibles/Stuff/KnightHelmet_BP.DeStun` (`self.HelmetRef`)))))))

(fn `UserConstructionScript`)