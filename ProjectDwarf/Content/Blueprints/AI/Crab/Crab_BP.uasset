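; Crab_BP is an AI crab that paces sideways, back and forth along its own right vector.
; Every Tick it applies low-scale movement input to the right or left, based on the ChangeDirection flag.
; A looping timer started on BeginPlay flips that flag at the TimerChangeDirection interval.
; BeginPlay also caches CameraBP from GameMode_BP, though the graph never uses it, and skips the timer if that cast fails.
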(event `self.ReceiveBeginPlay`
  (bind _asgame_mode_bp (cast `/Game/Blueprints/GameMode_BP` (`GameplayStatics.GetGameMode`)))
  (set `self.Camera_BP` (`/Game/Blueprints/GameMode_BP.CameraBP` _asgame_mode_bp))
  (`KismetSystemLibrary.K2_SetTimerDelegate` (delegate `ChangeDirectionEvent`) (`self.TimerChangeDirection`) true))

(event `self.ReceiveTick`
  (params (DeltaSeconds :type "Float (single-precision)"))
  (if (`self.ChangeDirection`)
    (`self.AddMovementInput` (`KismetMathLibrary.GetRightVector` (`self.K2_GetActorRotation`)) 0.2)
    (else
      (`self.AddMovementInput` (`KismetMathLibrary.GetRightVector` (`self.K2_GetActorRotation`)) -0.2))))

(event `ChangeDirectionEvent`
  (if (`self.ChangeDirection`)
    (set `self.ChangeDirection` false)
    (else
      (set `self.ChangeDirection` true))))

(fn `UserConstructionScript`)