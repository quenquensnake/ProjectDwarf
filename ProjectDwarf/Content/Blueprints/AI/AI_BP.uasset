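; AI character Blueprint that takes axe hits from the player and collapses when its health runs out.
; A capsule overlap with an Axe_BP removes one Health only while the player character's SlashSword flag is set.
; When Health reaches exactly zero, the skeletal mesh switches to physics simulation as a ragdoll death.
; A separate Run event sets the character's max walk speed.
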(event `Run`
  (set `CharacterMovementComponent.MaxWalkSpeed` 250.0 (`self.CharacterMovement`)))

(event `self.CapsuleComponent.OnComponentBeginOverlap`
  (params (OverlappedComponent :type "PrimitiveComponent Object Reference") (OtherActor :type "Actor Object Reference") (OtherComp :type "PrimitiveComponent Object Reference") (OtherBodyIndex :type Integer) (bFromSweep :type Boolean) (SweepResult :type "HitResult Structure (by ref)"))
  (bind _health (`self.Health`))
  ;[1 1 1] Getting damaged
  (bind _asaxe_bp (cast `/Game/Blueprints/Axe_BP` OtherActor))
  (bind _asplayer_bp (cast `/Game/Blueprints/Player_BP` (`GameplayStatics.GetPlayerCharacter` (`/Game/Blueprints/Axe_BP.PlayerOwner` _asaxe_bp))))
  (if (`/Game/Blueprints/Player_BP.SlashSword` _asplayer_bp)
    (`/Engine/EditorBlueprintResources/StandardMacros.DecrementInt` _health
      (:`  `
        (if (== _health 0)
          (`PrimitiveComponent.SetSimulatePhysics` (`self.Mesh`) true))))))

(fn `UserConstructionScript`)