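; AI controller for the flying Fly enemy that drives its behavior tree and feeds it the player as a follow target.
; On possessing a Fly pawn it runs the Fly behavior tree and blackboard, storing the controller itself under the SelfActor key.
; AI perception updates set the follow-target key to the player when sensed and clear it when lost.
; An unconnected node that would set the movement-type enum never runs.
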(event `self.OnPossess`
  (params (PossessedPawn :type "Pawn Object Reference"))
  (cast `/Game/Blueprints/AI/Fly/Fly_AI_BP` PossessedPawn)
  (`self.RunBehaviorTree` "/Game/Blueprints/AI/Fly/Fly_AI_BT.Fly_AI_BT")
  (`self.UseBlackboard` "/Game/Blueprints/AI/Fly/Fly_AI_BB.Fly_AI_BB")
  (`BlackboardComponent.SetValueAsObject` (`AIBlueprintHelperLibrary.GetBlackboard` null) "SelfActor Fly" self))

(event `self.AIPerception.OnTargetPerceptionUpdated`
  (params (Actor :type "Actor Object Reference") (Stimulus :type "AIStimulus Structure"))
  (bind _asplayer_bp (cast `/Game/Blueprints/Player_BP` Actor))
  (set `self.Player_ref Fly AIC` null)
  (bind _output_get (set `self.CanSeePlayer` (`.bSuccessfullySensed` (break `AIStimulus` Stimulus))))
  (if (== _output_get true)
    (`BlackboardComponent.SetValueAsObject` (`AIBlueprintHelperLibrary.GetBlackboard` null) "TargetToFollow Fly" _asplayer_bp)
    (else
      (`BlackboardComponent.SetValueAsObject` (`AIBlueprintHelperLibrary.GetBlackboard` null) "TargetToFollow Fly" null))))

(fn `UserConstructionScript`)