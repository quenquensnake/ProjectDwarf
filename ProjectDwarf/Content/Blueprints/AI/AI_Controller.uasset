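; AI controller for the AI_BP monster, which targets players it perceives.
; On possession it stores the monster, runs the AI_BT behavior tree and sets up its blackboard; a Run event forwards to the monster.
; Perception updates set the TargetToFollow blackboard key to a sensed Player_BP and clear it when sensing fails.
; An alternative perception handler and the two-player UpdatePlayersSaw tracking are left disconnected.
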(event `self.OnPossess`
  (params (PossessedPawn :type "Pawn Object Reference"))
  (bind _asai_bp (cast `/Game/Blueprints/AI/AI_BP` PossessedPawn))
  (set `self.Monster` _asai_bp)
  (`self.RunBehaviorTree` "/Game/Blueprints/AI/AI_BT.AI_BT")
  (`self.UseBlackboard` "/Game/Blueprints/AI/AIBlackBoard.AIBlackBoard")
  (`BlackboardComponent.SetValueAsObject` (`AIBlueprintHelperLibrary.GetBlackboard` null) "SelfActor" self))

(event `Run`
  (`/Game/Blueprints/AI/AI_BP.Run` (`self.Monster`)))

(event `self.AIPerception.OnTargetPerceptionUpdated`
  (params (Actor :type "Actor Object Reference") (Stimulus :type "AIStimulus Structure"))
  (bind _asplayer_bp (cast `/Game/Blueprints/Player_BP` Actor))
  (set `self.Player_ref` _asplayer_bp)
  (`KismetSystemLibrary.PrintString` (`KismetSystemLibrary.GetDisplayName` _asplayer_bp))
  (bind _output_get (set `self.CanSeePlayer` (`.bSuccessfullySensed` (break `AIStimulus` Stimulus))))
  (if (== _output_get true)
    (`BlackboardComponent.SetValueAsObject` (`AIBlueprintHelperLibrary.GetBlackboard` null) "TargetToFollow" _asplayer_bp)
    (else
      (`BlackboardComponent.SetValueAsObject` (`AIBlueprintHelperLibrary.GetBlackboard` null) "TargetToFollow" null))))

(fn `UpdatePlayersSaw`
  (params (Players :type "Array of Actor Object Reference"))
  (locals (Nobody :type Boolean))
  (`KismetArrayLibrary.Array_Clear` (`self.ArrayOfPlayers`))
  (for _array_element Players
    (bind _asplayer_bp (cast `/Game/Blueprints/Player_BP` _array_element))
    (`KismetArrayLibrary.Array_AddUnique` (`self.ArrayOfPlayers`) _asplayer_bp)
    (`/Engine/EditorBlueprintResources/StandardMacros.IsValid` _array_element
      (:`Is Valid`
        (`BlackboardComponent.SetValueAsObject` (`AIBlueprintHelperLibrary.GetBlackboard` null) "Player1" (`|GetArrayItem` (`self.ArrayOfPlayers`)))
        (`BlackboardComponent.SetValueAsObject` (`AIBlueprintHelperLibrary.GetBlackboard` null) "Player2" (`|GetArrayItem` (`self.ArrayOfPlayers`) 1)))))
  (if (== (`KismetArrayLibrary.Array_Length` Players) 0)
    (`KismetArrayLibrary.Array_Clear` (`self.ArrayOfPlayers`))
    (`KismetSystemLibrary.PrintString` "CLEAR")))

(fn `UserConstructionScript`)