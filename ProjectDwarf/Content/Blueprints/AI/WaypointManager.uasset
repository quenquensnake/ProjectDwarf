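; Level manager that assigns patrol waypoint routes to AI actors when play begins.
; On BeginPlay it finds actors tagged "AI" and matches their controllers against the AI entries in each Pathway element.
; Depending on whether the path is walkable or flyable, it copies waypoints, start point and wait time into the AI_Controller or Fly_AI_Controller_BP.
; It only hands over data; the controllers receive it for their own use.
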(event `self.ReceiveBeginPlay`
  (bind _outactors (`GameplayStatics.GetAllActorsWithTag` "AI"))
  (for _array_element _outactors
    (for (_array_element_2 _array_index) (`self.Pathway`)
      (set `self.IndexStruct` _array_index)
      (bind (_enum_ai _waypoints _ai) (break `/Game/Blueprints/AI/Waypoint_Struct` _array_element_2))
      (switch `/Game/Blueprints/AI/Enum_AI` _enum_ai
        (:`NewEnumerator0`
          (for _array_element_3 _ai
            (bind (_aiactor _aistart _aiwaittime) (break `/Game/Blueprints/AI/Start_AI` _array_element_3))
            (bind _returnvalue (`AIBlueprintHelperLibrary.GetAIController` _array_element))
            (if (== (`AIBlueprintHelperLibrary.GetAIController` _aiactor) _returnvalue)
              (bind _asai_controller (cast `/Game/Blueprints/AI/AI_Controller` _returnvalue))
              (set `/Game/Blueprints/AI/AI_Controller.Waypoints Actor AIC` _waypoints _asai_controller)
              (set `/Game/Blueprints/AI/AI_Controller.Waypoint to Start AIC` _aistart _asai_controller)
              (set `/Game/Blueprints/AI/AI_Controller.Time to Wait AIC` _aiwaittime _asai_controller)
              (set `self.Enum_AI` "NewEnumerator0"))))
        (:`NewEnumerator1`
          (for _array_element_4 _ai
            (bind (_aiactor_2 _aistart_2 _aiwaittime_2) (break `/Game/Blueprints/AI/Start_AI` _array_element_4))
            (if (== (`AIBlueprintHelperLibrary.GetAIController` _aiactor_2) _returnvalue)
              (bind _asfly_ai_controller_bp (cast `/Game/Blueprints/AI/Fly/Fly_AI_Controller_BP` _returnvalue))
              (set `/Game/Blueprints/AI/Fly/Fly_AI_Controller_BP.Waypoints Actor Fly AIC` _waypoints _asfly_ai_controller_bp)
              (set `/Game/Blueprints/AI/Fly/Fly_AI_Controller_BP.Waypoint to Start Fly AIC` _aistart_2 _asfly_ai_controller_bp)
              (set `/Game/Blueprints/AI/Fly/Fly_AI_Controller_BP.Time to Wait Fly AIC` _aiwaittime_2 _asfly_ai_controller_bp)
              (set `self.Enum_AI` "NewEnumerator1"))))))))

(fn `UserConstructionScript`)