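; Aiming component for the grappling hook that auto-selects what the owner can target.
; On BeginPlay it caches all ITargetable actors and the owner's Graplin_BP component.
; While the grapple is in its first state, each Tick picks the target closest to the owner's forward vector within distance and angle limits.
; It toggles target feedback and passes target and type to Graplin_BP; TrySetLock maintains a separate Locking flag.
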(event `self.ReceiveBeginPlay`
  (`self.RetrieveTargets`)
  (bind _output_get (set `self.owner` (`self.GetOwner`)))
  (set `self.GraplinBp_Ref` (`Actor.GetComponentByClass` _output_get "/Game/Blueprints/Graplin/Graplin_BP.Graplin_BP_C")))

(event `self.ReceiveTick`
  (params (DeltaSeconds :type "Float (single-precision)"))
  (if (`|EnumEquality` (`/Game/Blueprints/Graplin/Graplin_BP.State` (`self.GraplinBp_Ref`)) "NewEnumerator0")
    (bind _target (`self.PickTarget`))
    (`self.SetTarget` _target)
    (bind _output_get (set `/Game/Blueprints/Graplin/Graplin_BP.Target` _target (`self.GraplinBp_Ref`)))
    (bind _asitargetable (cast `/Game/Blueprints/Graplin/ITargetable` _output_get))
    (bind _type (`/Game/Blueprints/Graplin/ITargetable.GetTargetType` _asitargetable))
    (set `/Game/Blueprints/Graplin/Graplin_BP.TargetType` _type (`self.GraplinBp_Ref`))))

(fn `PickTarget`
  (returns (target :type "Actor Object Reference"))
  (locals (bestAngle :type "Float (double-precision)") (newTarget :type "Actor Object Reference"))
  (bind _owner (`self.owner`))
  (set `local.newTarget` null)
  (set `local.bestAngle` 360.0)
  (for _array_element (`self.Targets`)
    (bind _actor (`/Game/Blueprints/Graplin/ITargetable.GetActor` _array_element))
    (if (<= (`Actor.GetDistanceTo` _actor (`self.owner`)) (`self.DistanceRange`))
      (bind _angle (`/Game/Blueprints/Catchable/Tools_BPL.Angle Between Two Vectors` (- (`Actor.K2_GetActorLocation` _actor) (`Actor.K2_GetActorLocation` _owner)) (`Actor.GetActorForwardVector` _owner)))
      (if (< _angle (`self.AngleRange`))
        (if (< _angle (`local.bestAngle`))
          (set `local.bestAngle` _angle)
          (set `local.newTarget` _actor)))))
  (return (`local.newTarget`)))

(fn `RetrieveTargets`
  (bind _outactors (`GameplayStatics.GetAllActorsWithInterface` "/Game/Blueprints/Graplin/ITargetable.ITargetable_C"))
  (for _array_element _outactors
    (bind _asitargetable (cast `/Game/Blueprints/Graplin/ITargetable` _array_element))
    (`KismetArrayLibrary.Array_AddUnique` (`self.Targets`) _asitargetable))
  (`KismetSystemLibrary.PrintString` (`KismetStringLibrary.Concat_StrStr` (`KismetStringLibrary.Conv_IntToString` (`KismetArrayLibrary.Array_Length` (`self.Targets`))) " targets found")))

(fn `SetTarget`
  (params (newTarget :type "Actor Object Reference"))
  (if (`KismetSystemLibrary.IsValid` (`self.Target`))
    (bind _asitargetable (cast `/Game/Blueprints/Graplin/ITargetable` (`self.Target`))
      (:`then`
        (`/Game/Blueprints/Graplin/ITargetable.SetFeedback` _asitargetable false))
      (:`CastFailed`
        _)))
  (if (`KismetSystemLibrary.IsValid` newTarget)
    (bind _asitargetable_2 (cast `/Game/Blueprints/Graplin/ITargetable` newTarget)
      (:`then`
        (`/Game/Blueprints/Graplin/ITargetable.SetFeedback` _asitargetable_2 true))
      (:`CastFailed`
        _))
    (set `self.Target` newTarget)))

(fn `TrySetLock`
  (params (value :type Boolean))
  (if value
    (if (and (not (`self.Locking`)) (`KismetSystemLibrary.IsValid` (`self.Target`)))
      (set `self.Locking` true))
    (elif (`self.Locking`)
      (set `self.Locking` false))))