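; TargetFeedBack_BP is a target feedback marker in the Graplin folder, with a static mesh and a widget.
; BeginPlay raises the mesh by a Z offset and starts a Hover timeline that restarts when finished.
; The hover-driven widget movement is disconnected, so it never runs.
; SetOffSetZ stores a new offset and adds it to the mesh position, while SetActive shows or hides the widget.
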(event `self.ReceiveBeginPlay`
  (`SceneComponent.K2_AddLocalOffset` (`self.StaticMesh`) (`KismetMathLibrary.MakeVector` 0.0 0.0 (`self.OffsetZ`)) false false)
  (bind (_direction _position) (`Timeline|Hover` :!label _label)
    (:`Finished`
      (`TimelineComponent.Reverse` (`self.Hover`))
      (goto _label :!via `PlayFromStart`))))

(fn `SetActive`
  (params (active :type Boolean))
  (`SceneComponent.SetHiddenInGame` (`self.Widget`) (not active) false))

(fn `SetOffSetZ`
  (params (offset :type "Float (double-precision)"))
  (bind _output_get (set `self.OffsetZ` offset))
  (`SceneComponent.K2_AddLocalOffset` (`self.StaticMesh`) (`KismetMathLibrary.MakeVector` 0.0 0.0 _output_get) false false))

(fn `UserConstructionScript`)