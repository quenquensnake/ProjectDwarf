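; Actor component, filed under Graplin, that sets up its owning actor as a target with its own target widget.
; On BeginPlay it creates the widget and assigns it to the first of the owner's widget components tagged "Target".
; It also stores references to the owner, the widget and a primitive component found on the owner; Tick does nothing.
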(event `self.ReceiveBeginPlay`
  (set `self.TargetActor` (`self.GetOwner`))
  (bind _returnvalue (`|CreateWidget` "/Game/Blueprints/Graplin/TargetWidget.TargetWidget_C"))
  (bind _output_get (set `self.TargetWidget` _returnvalue))
  (for _array_element (`Actor.K2_GetComponentsByClass` (`self.TargetActor`) "/Script/UMG.WidgetComponent")
    (if (`self.ComponentHasTag` _array_element "Target")
      (`WidgetComponent.SetWidget` _array_element _output_get)
      (break)))
  (set `self.TargetPrimitiveComponent` (`Actor.GetComponentByClass` (`self.TargetActor`) "/Script/Engine.PrimitiveComponent")))

(event `self.ReceiveTick`
  (params (DeltaSeconds :type "Float (single-precision)")))