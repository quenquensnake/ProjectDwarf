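; Prop actor in the Graplin folder that acts as a target, exposing itself, its target type and its availability.
; SetFeedback shows or hides its TargetComponent as a visual cue and returns true.
; The getters return stored values or self, event and construction graphs are empty, and IsAvailable contains unconnected leftover feedback and debug-print nodes.
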(fn `GetActor`
  (returns (Actor :type "Actor Object Reference"))
  (return self))

(fn `GetTargetType`
  (returns (type :type "/Game/Blueprints/Graplin/TargetType Enum"))
  (return (`self.TargetType`)))

(fn `IsAvailable`
  (returns (available :type Boolean))
  (return (`self.Available`)))

(fn `SetFeedback`
  (params (enabled :type Boolean))
  (returns (success :type Boolean))
  (`/Game/Blueprints/Graplin/TargetComponent.SetVisible` (`self.TargetComponent`) enabled)
  (return true))

(fn `UserConstructionScript`)