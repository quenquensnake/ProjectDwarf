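; Grappling hook component that drives the owner's Cable component to throw a line and pull in actors tagged "Catchable".
; Tick runs a state machine: Idle highlights the catchable nearest the forward direction within an angle limit, using icons spawned at BeginPlay.
; TryThrowGraplin spawns cable-end actors on the target, or ahead when none exists, then time-based lerps move the cable end and reel catchables in.
; InterruptThrow is a stub, and the line-trace launch is unreachable.
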(event `self.ReceiveBeginPlay`
  ;[1 1 1] BeginPlay
  (bind _output_get (set `self.Owner` (`self.GetOwner`)))
  (bind _output_get_2 (set `self.Cable` (`Actor.GetComponentByClass` _output_get "/Script/CableComponent.CableComponent")))
  (`SceneComponent.SetVisibility` _output_get_2 false false)
  (set `self.lerp` 0.0)
  (set `self.State` "NewEnumerator0")
  (`self.InitWidgets`)
  (bind _returnvalue (`|SpawnActorFromClass` "/Game/Blueprints/Graplin/GraplinHook.GraplinHook_C" (`Actor.GetTransform` (`self.Owner`)) "Undefined" "OverrideRootScale"))
  (`Actor.SetActorHiddenInGame` _returnvalue true)
  (`CableComponent.SetAttachEndTo` (`self.Cable`) _returnvalue "None" "None"))

(event `self.ReceiveTick`
  (params (DeltaSeconds :type "Float (single-precision)"))
  ;[1 1 1] Update
  (switch `/Game/Blueprints/Graplin/GraplinState` (`self.State`)
    (:`NewEnumerator0`
      (bind _output_target (`self.PickTarget`))
      (set `self.Target` _output_target)
      (`self.SetWidgetTargetted`))
    (:`NewEnumerator1`
      (`self.ThrowingGraplin`))
    (:`NewEnumerator2`
      (`self.RetreiveCatchable`))))

(fn `DestroyAttach`
  (`Actor.K2_DestroyActor` (`self.CableEndAttach`))
  (set `self.CableEndAttach` null))

(fn `IncrementLerp`
  (returns (lerp :type "Float (double-precision)"))
  (bind _output_get (set `self.lerp` (+ (`self.lerp`) (`GameplayStatics.GetWorldDeltaSeconds`))))
  (return _output_get))

(fn `InitWidgets`
  (bind _outactors (`GameplayStatics.GetAllActorsWithTag` "Catchable"))
  (for _array_element _outactors
    (bind _returnvalue (`|SpawnActorFromClass` "/Game/Blueprints/Catchable/Target_UI_BP.Target_UI_BP_C" (`KismetMathLibrary.Conv_VectorToTransform` (`KismetMathLibrary.MakeVector` 0.0 0.0 0.0)) "Undefined" "OverrideRootScale" _array_element))
    (`Actor.K2_AttachToActor` _returnvalue _array_element "grab_icon_location" "KeepRelative" "KeepRelative" "KeepRelative" true)
    (`BlueprintMapLibrary.Map_Add` (`self.dicWidgets`) _array_element _returnvalue)
    (`Actor.SetActorHiddenInGame` _returnvalue true)))

(fn `InterruptThrow`
  (`KismetSystemLibrary.PrintString` "INTERRUPT"))

(fn `PickTarget`
  (returns (`Output Target` :type "Actor Object Reference"))
  (locals (newTarget :type "Actor Object Reference") (bestAngle :type "Float (double-precision)"))
  (bind _owner (`self.Owner`))
  (set `local.bestAngle` 360.0)
  (bind _keys (`BlueprintMapLibrary.Map_Keys` (`self.dicWidgets`)))
  (for _array_element _keys
    (bind _angle (`/Game/Blueprints/Catchable/Tools_BPL.Angle Between Two Vectors` (- (`Actor.K2_GetActorLocation` _owner) (`Actor.K2_GetActorLocation` _array_element)) (* (`Actor.GetActorForwardVector` _owner) -1)))
    (if (< _angle (`local.bestAngle`))
      (set `local.bestAngle` _angle)
      (set `local.newTarget` _array_element)))
  ;[1 1 1] Loop Completed
  (if (< (`local.bestAngle`) (`self.Angle_Range`))
    (return (`local.newTarget`))
    (else
      (return null))))

(fn `RetreiveCatchable`
  (bind _target (`self.Target`))
  (bind _lerp (`self.IncrementLerp`))
  (`/Game/Blueprints/Catchable/Tools_BPL.LerpActor` _target _target (`self.Owner`) _lerp)
  (if (<= (`Actor.GetDistanceTo` (`self.Target`) (`self.Owner`)) 250.0)
    (set `self.State` "NewEnumerator0")
    (`self.DestroyAttach`)
    (`SceneComponent.SetVisibility` (`self.Cable`) false false)))

(fn `SetWidgetTargetted`
  (bind _keys (`BlueprintMapLibrary.Map_Keys` (`self.dicWidgets`)))
  (for (_array_element _array_index) _keys
    (if (== _array_element (`self.Target`))
      (bind _values (`BlueprintMapLibrary.Map_Values` (`self.dicWidgets`)))
      (`Actor.SetActorHiddenInGame` (`|GetArrayItem` _values _array_index) false)
      (else
        (bind _values_2 (`BlueprintMapLibrary.Map_Values` (`self.dicWidgets`)))
        (`Actor.SetActorHiddenInGame` (`|GetArrayItem` _values_2 _array_index) true)))))

(fn `ThrowingGraplin`
  (bind _cable (`self.Cable`))
  (bind _cableendattach (`self.CableEndAttach`))
  (bind _lerp (`self.IncrementLerp`))
  (`/Game/Blueprints/Catchable/Tools_BPL.LerpActor` _cableendattach _cableendattach (`self.Target`) _lerp)
  (`self.UpdateCableLenght` (`Actor.K2_GetActorLocation` (`self.CableEndAttach`)))
  (if (>= (`self.lerp`) 1.0)
    (switch `/Game/Blueprints/Graplin/TargetType` (`self.TargetType`)
      (:`NewEnumerator4`
        (set `self.State` "NewEnumerator0")
        (`SceneComponent.SetVisibility` _cable false false)
        (set `CableComponent.CableLength` 0.0 _cable)
        (`self.DestroyAttach`)
        (if (`|EnumEquality` (`self.TargetType`) "NewEnumerator4")
          (`Actor.K2_DestroyActor` (`self.Target`))))
      (:`NewEnumerator1`
        (`self.TriggerCatch`)
        (`KismetSystemLibrary.PrintString` "MDR")))))

(fn `TriggerCatch`
  (returns (`Out Success` :type Boolean))
  (set `self.lerp` 0.0)
  (set `self.State` "NewEnumerator2")
  (return true))

(fn `TryThrowGraplin`
  (returns (`Out Success` :type Boolean))
  (bind _owner (`self.Owner`))
  ;[1 1 1] Check Idle
  (if (`|EnumEquality` (`self.State`) "NewEnumerator0")
    (set `self.State` "NewEnumerator1")
    (set `self.lerp` 0.0)
    (`SceneComponent.SetVisibility` (`self.Cable`) true false)
    (if (`KismetSystemLibrary.IsValid` (`self.Target`))
      ;[1 1 1] There is a target
      (set `self.TargetType` "NewEnumerator1")
      (bind _returnvalue (`|SpawnActorFromClass` "/Game/Blueprints/Graplin/CableAttachEnd.CableAttachEnd_C" (`Actor.GetTransform` (`self.Target`)) "Undefined" "OverrideRootScale"))
      (bind _output_get (set `self.CableEndAttach` _returnvalue))
      (`CableComponent.SetAttachEndTo` (`self.Cable`) _output_get "None" "None")
      (return true)
      (else
        ;[1 1 1] There are no target
        (bind _returnvalue_2 (`|SpawnActorFromClass` "/Game/Blueprints/Graplin/CableAttachEnd.CableAttachEnd_C" (`KismetMathLibrary.Conv_VectorToTransform` (+ (`Actor.K2_GetActorLocation` _owner) (* (`Actor.GetActorForwardVector` _owner) 300))) "Undefined" "OverrideRootScale"))
        (set `self.Target` _returnvalue_2)
        (set `self.TargetType` "NewEnumerator4")
        (bind _returnvalue_3 (`|SpawnActorFromClass` "/Game/Blueprints/Graplin/CableAttachEnd.CableAttachEnd_C" (`Actor.GetTransform` (`self.Owner`)) "Undefined" "OverrideRootScale"))
        (bind _output_get_2 (set `self.CableEndAttach` _returnvalue_3))
        (`CableComponent.SetAttachEndTo` (`self.Cable`) _output_get_2 "None" "None")
        (return true)))
    (else
      (return false))))

(fn `UpdateCableLenght`
  (params (TargetPos :type "Vector Structure"))
  (set `CableComponent.CableLength` (`KismetMathLibrary.VSize` (- TargetPos (`Actor.K2_GetActorLocation` (`self.CableEndAttach`)))) (`self.Cable`)))