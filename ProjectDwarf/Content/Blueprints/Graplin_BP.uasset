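; Grappling hook Blueprint that works on its owner's cable component, with target selection live and the launch logic left disconnected.
; At BeginPlay it hides the cable and attaches a hidden icon actor to each "Catchable" actor.
; TryGrapnel picks a target by angle to the owner's forward vector and reveals only its icon.
; Tick can lerp the owner to the cable's end, but only the unwired line-trace launch starts that pull.
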(event `self.ReceiveBeginPlay`
  ;[1 1 1] BeginPlay
  (bind _output_get (set `self.Owner` (`self.GetOwner`)))
  (bind _output_get_2 (set `self.Cable` (`Actor.GetComponentByClass` _output_get "/Script/CableComponent.CableComponent")))
  (`SceneComponent.SetVisibility` _output_get_2 false false)
  (set `self.lerp` 0.0)
  (bind _output_get_3 (set `self.isReaching` false))
  (set `self.isCatching` _output_get_3)
  (`self.InitWidgets`))

(event `TryGrapnel`
  (bind _output_target (`self.PickTarget`))
  (set `self.Target` _output_target)
  (`self.SetWidgetTargetted`))

(event `self.ReceiveTick`
  (params (DeltaSeconds :type "Float (single-precision)"))
  (`self.UpdateWidgets`)
  (if (`self.isReaching`)
    (bind _output_get (set `self.lerp` (+ (`self.lerp`) (`GameplayStatics.GetWorldDeltaSeconds`))))
    (if (>= _output_get 1.0)
      (`Actor.K2_SetActorLocation` (`self.Owner`) (`Actor.K2_GetActorLocation` (`self.CableEndAttach`)) false false)
      (set `self.isReaching` false)
      (`SceneComponent.SetVisibility` (`self.Cable`) false false)
      (`Actor.K2_DestroyActor` (`self.CableEndAttach`))
      (else
        (`Actor.K2_SetActorLocation` (`self.Owner`) (`KismetMathLibrary.VLerp` (`Actor.K2_GetActorLocation` (`self.Owner`)) (`Actor.K2_GetActorLocation` (`self.CableEndAttach`)) _output_get) false false)
        (`self.SetCableLenght` (`Actor.K2_GetActorLocation` (`self.CableEndAttach`)))))))

(fn `Catching`
  (locals (NewLocalVar_0 :type "Float (double-precision)")))

(fn `InitWidgets`
  (bind _outactors (`GameplayStatics.GetAllActorsWithTag` "Catchable"))
  (for _array_element _outactors
    (bind _returnvalue (`|SpawnActorFromClass` "/Game/Blueprints/Catchable/Target_UI_BP.Target_UI_BP_C" (`KismetMathLibrary.Conv_VectorToTransform` (`KismetMathLibrary.MakeVector` 0.0 0.0 0.0)) "Undefined" "OverrideRootScale" _array_element))
    (`Actor.K2_AttachToActor` _returnvalue _array_element "grab_icon_location" "KeepRelative" "KeepRelative" "KeepRelative" true)
    (`BlueprintMapLibrary.Map_Add` (`self.dicWidgets`) _array_element _returnvalue)
    (`Actor.SetActorHiddenInGame` _returnvalue true)))

(fn `PickTarget`
  (returns (`Output Target` :type "Actor Object Reference"))
  (locals (newTarget :type "Actor Object Reference") (bestAngle :type "Float (double-precision)"))
  (bind _owner (`self.Owner`))
  (set `local.bestAngle` 360.0)
  (bind _keys (`BlueprintMapLibrary.Map_Keys` (`self.dicWidgets`)))
  (for _array_element _keys
    (bind _angle (`/Game/Blueprints/Catchable/Tools_BPL.Angle Between Two Vectors` (- (`Actor.K2_GetActorLocation` _owner) (`Actor.K2_GetActorLocation` _array_element)) (`Actor.GetActorForwardVector` _owner)))
    (if (< _angle (`local.bestAngle`))
      (set `local.bestAngle` _angle)
      (set `local.newTarget` _array_element)))
  ;[1 1 1] Loop Completed
  (if (< (`local.bestAngle`) (`self.Angle_Range`))
    (return (`local.newTarget`))))

(fn `SetCableLenght`
  (params (TargetPos :type "Vector Structure"))
  (set `CableComponent.CableLength` (`KismetMathLibrary.VSize` (- TargetPos (`Actor.K2_GetActorLocation` (`self.Owner`)))) (`self.Cable`)))

(fn `SetWidgetTargetted`
  (bind _keys (`BlueprintMapLibrary.Map_Keys` (`self.dicWidgets`)))
  (for (_array_element _array_index) _keys
    (if (== _array_element (`self.Target`))
      (bind _values (`BlueprintMapLibrary.Map_Values` (`self.dicWidgets`)))
      (`Actor.SetActorHiddenInGame` (`|GetArrayItem` _values _array_index) false)
      (else
        (bind _values_2 (`BlueprintMapLibrary.Map_Values` (`self.dicWidgets`)))
        (`Actor.SetActorHiddenInGame` (`|GetArrayItem` _values_2 _array_index) true)))))

(fn `UpdateWidgets`)