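; Tools_BPL is a function library of small math and actor helpers.
; Angle functions measure degrees between vectors flattened onto the XY plane, including from one actor's forward vector to the direction of another actor.
; Lerp helpers compute a point between two actors' locations or move an actor there without sweeping.
; Other checks report whether two values avoid opposite signs and whether a 2D input falls inside a fixed radial dead zone.
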(fn `Angle Between Two Actors`
  (params (Actor1 :type "Actor Object Reference") (Actor2 :type "Actor Object Reference"))
  (returns (Angle :type "Float (double-precision)"))
  (bind _angle (`self.Angle Between Two Vectors` (`Actor.GetActorForwardVector` Actor1) (- (`Actor.K2_GetActorLocation` Actor2) (`Actor.K2_GetActorLocation` Actor1)) true))
  (return _angle))

(fn `Angle Between Two Vectors`
  (params (A :type "Vector Structure") (B :type "Vector Structure") (absolute :type Boolean))
  (returns (angle :type "Float (double-precision)"))
  (bind _returnvalue (`KismetMathLibrary.DegAcos` (`KismetMathLibrary.Dot_VectorVector` (`KismetMathLibrary.Normal` (`KismetMathLibrary.MakeVector` A_X A_Y)) (`KismetMathLibrary.Normal` (`KismetMathLibrary.MakeVector` B_X B_Y)))))
  ;[1 1 1] Return the angle between two vectors in degrees
  (if absolute
    (return (`KismetMathLibrary.Abs` _returnvalue))
    (else
      (return _returnvalue))))

(fn `CheckDeadZone`
  (params (x :type "Float (double-precision)") (y :type "Float (double-precision)"))
  (returns (`In Dead Zone` :type Boolean))
  (return (<= (`KismetMathLibrary.VSize2D` (`KismetMathLibrary.MakeVector2D` x y)) 0.2)))

(fn `GetLerpPosition`
  (params (From :type "Actor Object Reference") (To :type "Actor Object Reference") (LerpValue :type "Float (double-precision)"))
  (returns (Result :type "Vector Structure"))
  (return (`KismetMathLibrary.VLerp` (`Actor.K2_GetActorLocation` From) (`Actor.K2_GetActorLocation` To) LerpValue)))

(fn `LerpActor`
  (params (ActorToMove :type "Actor Object Reference") (From :type "Actor Object Reference") (To :type "Actor Object Reference") (lerp :type "Float (double-precision)"))
  (`Actor.K2_SetActorLocation` ActorToMove (`KismetMathLibrary.VLerp` (`Actor.K2_GetActorLocation` From) (`Actor.K2_GetActorLocation` To) lerp) false false))

(fn `SameSign`
  (params (value1 :type "Float (double-precision)") (value2 :type "Float (double-precision)"))
  (returns (Same :type Boolean))
  (if (and (< value2 0.0) (> value1 0.0))
    (return false)
    (elif (and (< value1 0.0) (> value2 0.0))
      (return false)
      (else
        (return true)))))