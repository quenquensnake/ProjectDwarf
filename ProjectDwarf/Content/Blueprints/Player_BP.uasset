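; Player character Blueprint for a dwarf with an axe, grapnel, fog horn and item pickup.
; Movement and facing follow CameraGame; Tick handles lock-on to the grapnel target and drops sprint to walking when input stops.
; GraplinBP and PlayerInteractionAC handle throws and interactions, while the horn impulses actors overlapping its box.
; Attacks replay one montage through a buffered save flag; staged combos are unreachable and the charged attack only prints.
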(event `self.ReceiveBeginPlay`
  ;[1 1 1] BeginPlay
  (bind _asdwarf_anim_blueprint (cast `/Game/Animations/DwarfAnimBlueprint` (`SkeletalMeshComponent.GetAnimInstance` (`self.Mesh`))))
  (bind _output_get (set `/Game/Animations/DwarfAnimBlueprint.IdPlayer` (`self.Id`) _asdwarf_anim_blueprint))
  (bind _returnvalue (`|SpawnActorFromClass` "/Game/Blueprints/Axe_BP.Axe_BP_C" (`SceneComponent.GetSocketTransform` (`self.Mesh`) "SpineSocket" "RTS_World") "AlwaysSpawn" "OverrideRootScale"))
  (bind _output_get_2 (set `self.Axe` _returnvalue))
  (set `/Game/Blueprints/Axe_BP.PlayerOwner` _output_get _output_get_2)
  (`SceneComponent.K2_AttachToComponent` (`self.GetComponentByClass` _output_get_2 "/Script/Engine.StaticMeshComponent") (`self.Mesh`) "SpineSocket" "SnapToTarget" "SnapToTarget" "SnapToTarget" true)
  (set `CharacterMovementComponent.MaxWalkSpeed` (`self.WalkSpeed`) (`self.CharacterMovement`)))

(event `InputAction|Jump`
  (params (Key :type "Key Structure" :default "AnyKey"))
  ;[1 1 1] Jump Control (This is curently garbage)
  (:`Pressed`
    (`CharacterMovementComponent.AddImpulse` (`self.CharacterMovement`) (0.0 0.0 300.0) true)))

(event `InputAction|Run`
  (params (Key :type "Key Structure" :default "AnyKey"))
  ;[1 1 1] RunControl
  (:`Pressed`
    (set `self.Running` true)
    (set `CharacterMovementComponent.MaxWalkSpeed` (`self.RunSpeed`) (`self.CharacterMovement`))))

(event `self.ReceiveTick`
  (params (DeltaSeconds :type "Float (single-precision)"))
  ;[1 1 1] EventTick
  (`self.TryLookAtTarget`)
  (`self.CheckMustStopRun`))

(event `InputAction|grapnel`
  (params (Key :type "Key Structure" :default "AnyKey"))
  ;[1 1 1] GraplinControl
  (:`Pressed`
    (bind _out_success (`/Game/Blueprints/Graplin/Graplin_BP.TryThrowGraplin` (`self.Graplin_BP`)))
    (if _out_success
      (bind _asdwarf_anim_blueprint (cast `/Game/Animations/DwarfAnimBlueprint` (`SkeletalMeshComponent.GetAnimInstance` (`self.Mesh`))))
      (set `/Game/Animations/DwarfAnimBlueprint.Launching` true _asdwarf_anim_blueprint)
      (`GameplayStatics.PlaySoundAtLocation` (select `int` (`KismetMathLibrary.RandomInteger` 3) :`0` "/Game/Sounds/Grapnel/throw_00.throw_00" :`1` "/Game/Sounds/Grapnel/throw_01.throw_01" :`2` "/Game/Sounds/Grapnel/throw_02.throw_02" :!type "SoundBase Object Reference") (`self.K2_GetActorLocation`)))))

(event `InputAction|Lock`
  (params (Key :type "Key Structure" :default "AnyKey"))
  ;[1 1 1] LockControl
  (:`Pressed`
    (`self.SetLock` true))
  (:`Released`
    (`self.SetLock` false)))

(event `InputAxis|MoveForward`
  (params (AxisValue :type "Float (single-precision)"))
  ;[1 1 1] Mouvements
  (`self.Move` (`KismetMathLibrary.MakeVector` 0.0 AxisValue)))

(event `InputAxis|MoveRight`
  (params (AxisValue :type "Float (single-precision)"))
  ;[1 1 1] Mouvements
  (`self.Move` (`KismetMathLibrary.MakeVector` AxisValue)))

(event `Key|LeftMouseButton`
  (params (Key :type "Key Structure" :default "AnyKey"))
  ;[1 1 1] Attack
  (:`Pressed`
    (set `self.attacking?` true)
    (`KismetSystemLibrary.Delay` 0.5)
    (set `self.attacking?` false)))

(event `InputAction|Interact`
  (params (Key :type "Key Structure" :default "AnyKey"))
  (bind _playerinteraction_ac (`self.PlayerInteraction_AC`))
  ;[1 1 1] PickUpItem
  (:`Pressed`
    (`/Game/Blueprints/Interaction/Interactibles/PlayerInteraction_AC.SetPlayerPickup` _playerinteraction_ac)
    (bind _selectedinteraction (`/Game/Blueprints/Interaction/Interactibles/PlayerInteraction_AC.SelectedInteraction` _playerinteraction_ac)
      (:`then`
        (`/Game/Blueprints/Interaction/Interactibles/Interaction_BP.Interact` _selectedinteraction self))
      (:`else`
        (bind _currentpickup (`/Game/Blueprints/Interaction/Interactibles/PlayerInteraction_AC.CurrentPickUp` _playerinteraction_ac)
          (:`then`
            (bind _bisdropped (`/Game/Blueprints/Interaction/Interactibles/PlayerInteraction_AC.DropPickUp` _playerinteraction_ac _currentpickup (`self.GetInputAxisValue`) (`self.GetInputAxisValue`)))
            (if _bisdropped
              (set `/Game/Blueprints/Interaction/Interactibles/PlayerInteraction_AC.CurrentPickUp` null _playerinteraction_ac)))
          (:`else`))))))

(event `Key|F`
  (params (Key :type "Key Structure" :default "AnyKey"))
  ;[1 1 1] Activate FogHorn
  (:`Pressed`
    (`PrimitiveComponent.SetCollisionEnabled` (`self.Box`) "QueryAndPhysics")
    ;[1 1 1] FogHorn
    (for _array_element (`PrimitiveComponent.GetOverlappingActors` (`self.Box`) null) :!label _label
      (bind _asprimitive_component (cast `PrimitiveComponent` (`self.K2_GetRootComponent` _array_element)))
      (`PrimitiveComponent.AddImpulse` _asprimitive_component (* (`self.GetActorForwardVector`) 5000.0) "None" false)))
  (:`Released`
    (`PrimitiveComponent.SetCollisionEnabled` (`self.Box`) "NoCollision")
    (goto _label)))

(event `InputAxis|LookX`
  (params (AxisValue :type "Float (single-precision)"))
  ;[1 1 1] LookAroundControl
  (if (and (!= (+ (`self.GetInputAxisValue`) (`self.GetInputAxisValue`)) 0.0) (not (`self.Locking`))) :!label _label_2
    (`self.TryLook` (`KismetMathLibrary.MakeVector` AxisValue (stale `InputAxis|LookY` AxisValue)))))

(event `InputAxis|LookY`
  (params (AxisValue :type "Float (single-precision)"))
  ;[1 1 1] LookAroundControl
  (goto _label_2))

(event `self.CapsuleComponent.OnComponentHit`
  (params (HitComponent :type "PrimitiveComponent Object Reference") (OtherActor :type "Actor Object Reference") (OtherComp :type "PrimitiveComponent Object Reference") (NormalImpulse :type "Vector Structure") (Hit :type "HitResult Structure (by ref)"))
  (bind _capsulecomponent (`self.CapsuleComponent`))
  (bind (_returnvalue_roll _returnvalue_pitch _returnvalue_yaw) (`KismetMathLibrary.BreakRotator` (`SceneComponent.K2_GetComponentRotation` _capsulecomponent)))
  (if (`self.CapsuleHasHit`)
    (`PrimitiveComponent.SetCollisionResponseToChannel` _capsulecomponent "ECC_Pawn" "ECR_Block")
    (`PrimitiveComponent.SetSimulatePhysics` _capsulecomponent false)
    (`SceneComponent.K2_SetWorldRotation` _capsulecomponent (`KismetMathLibrary.MakeRotator` _returnvalue_roll 0.0 _returnvalue_yaw) false false)
    (`CharacterMovementComponent.SetMovementMode` (`self.CharacterMovement`) "MOVE_Walking" 0)
    (set `self.CapsuleHasHit` false)))

(event `InputAction|Attack`
  (params (Key :type "Key Structure" :default "AnyKey"))
  ;[1 1 1] Combos
  (:`Pressed`
    (if (`self.SlashSword`) :!label _label
      (set `self.SaveAttack` true)
      (else
        (set `self.SaveAttack` true)
        (set `self.SlashSword` true :!label _label_2)
        (bind _returnvalue (`AnimInstance.Montage_Play` (`SkeletalMeshComponent.GetAnimInstance` (`self.Mesh`)) "/Game/Animations/Montages/Attack1Montage.Attack1Montage" 1.0 "MontageLength" 0.0))
        (`KismetSystemLibrary.Delay` _returnvalue)
        (set `self.SlashSword` false)))))

(event `Key|LeftMouseButton`
  (params (Key :type "Key Structure" :default "AnyKey"))
  ;[1 1 1] Combos
  (:`Pressed`
    (goto _label)))

(event `SaveComboAttack`
  ;[1 1 1] Combos
  (if (`self.SaveAttack`)
    (set `self.SaveAttack` false)
    (goto _label_2)))

(event `ResetCombo`
  ;[1 1 1] AttackButton
  (set `self.ComboCounter` 0)
  (set `self.SaveAttack` false)
  (set `self.SlashSword` false))

(event `CustomEvent`
  (params (DeltaSeconds :type "Float (double-precision)"))
  ;[1 1 1] ABSOLUTELY NOTHING
)

(event `Key|R`
  (params (Key :type "Key Structure" :default "AnyKey"))
  (bind _timeheld (`self.TimeHeld`))
  ;[1 1 1] ABSOLUTELY NOTHING
  (:`Pressed`
    (`/Engine/EditorBlueprintResources/StandardMacros.Gate` true :!via `Open` :!label _label_3
      (:`Exit`
        (set `self.TimeHeld` (+ 0.0 _timeheld)))))
  (:`Released`
    (if (>= _timeheld 2.0)
      (`KismetSystemLibrary.PrintString` "Charged attack"))
    (set `self.TimeHeld` 0.0)
    (goto _label_3 :!via `Close`)))

(fn `CheckMustStopRun`
  (returns (stopped :type Boolean))
  (if (and (`self.Running`) (and (== 0.0 (`self.GetInputAxisValue`)) (== (`self.GetInputAxisValue`) 0.0)))
    (set `self.Running` false)
    (set `CharacterMovementComponent.MaxWalkSpeed` (`self.WalkSpeed`) (`self.CharacterMovement`))
    (return true)
    (else
      (return false))))

(fn `Move`
  (params (Input :type "Vector Structure"))
  (bind _cameragame (`self.CameraGame`))
  (bind (_returnvalue_roll _returnvalue_pitch _returnvalue_yaw) (`KismetMathLibrary.BreakRotator` (`SceneComponent.K2_GetComponentRotation` _cameragame)))
  (`self.AddMovementInput` (`KismetMathLibrary.Conv_RotatorToVector` (`SceneComponent.K2_GetComponentRotation` _cameragame)) Input_Y)
  (`self.AddMovementInput` (`KismetMathLibrary.GetRightVector` (`KismetMathLibrary.MakeRotator` 0.0 0.0 _returnvalue_yaw)) Input_X))

(fn `SetLock`
  (params (value :type Boolean))
  (if value
    (if (and (not (`self.Locking`)) (`KismetSystemLibrary.IsValid` (`/Game/Blueprints/Graplin/Graplin_BP.Target` (`self.Graplin_BP`))))
      (set `self.Locking` true))
    (elif (`self.Locking`)
      (set `self.Locking` false))))

(fn `TryLook`
  (params (Input :type "Vector Structure"))
  (bind (_returnvalue_roll _returnvalue_pitch _returnvalue_yaw) (`KismetMathLibrary.BreakRotator` (`SceneComponent.K2_GetComponentRotation` (`self.CameraGame`))))
  (`SceneComponent.K2_SetRelativeRotation` (`self.CapsuleComponent`) (`KismetMathLibrary.ComposeRotators` (`KismetMathLibrary.MakeRotator` 0.0 0.0 (`KismetMathLibrary.DegAtan2` Input_X Input_Y)) (`KismetMathLibrary.MakeRotator` 0.0 0.0 _returnvalue_yaw)) false false))

(fn `TryLookAtTarget`
  (bind (_returnvalue_roll _returnvalue_pitch _returnvalue_yaw) (`KismetMathLibrary.BreakRotator` (`KismetMathLibrary.FindLookAtRotation` (`self.K2_GetActorLocation`) (`self.K2_GetActorLocation` (`/Game/Blueprints/Graplin/Graplin_BP.Target` (`self.Graplin_BP`))))))
  (if (and (`self.Locking`) (`KismetSystemLibrary.IsValid` (`/Game/Blueprints/Graplin/Graplin_BP.Target` (`self.Graplin_BP`))))
    (`self.K2_SetActorRotation` (`KismetMathLibrary.MakeRotator` 0.0 0.0 _returnvalue_yaw))))

(fn `UserConstructionScript`
  (`SceneComponent.SetWorldScale3D` (`self.FogHornArrow`) (1.0 1.0 1.0)))