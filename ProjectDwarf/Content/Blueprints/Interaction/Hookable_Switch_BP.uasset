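; Hookable switch for the interaction system that shows an on or off state as a grappling hook activates or deactivates it.
; Activate and deactivate events play a metal ting, call the parent logic, then snap the mesh to an opposite tilt and swap its material.
; A separate Toogle function, not called within this graph, flips Active and switches the Visual material between active and disabled.
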(event `self.Activate_Hook`
  (bind _staticmesh1 (`self.StaticMesh1`))
  (`GameplayStatics.PlaySoundAtLocation` "/Game/Sounds/Grapnel/metal_ting.metal_ting" (`self.K2_GetActorLocation`))
  (`parent.Activate_Hook`)
  (`SceneComponent.K2_SetRelativeRotation` _staticmesh1 (struct :`Roll` 50.0) false false)
  (`PrimitiveComponent.SetMaterial` _staticmesh1 0 "/Game/Meshes/fbx_AssetsMap/GrapActivator/GrapActivatorON.GrapActivatorON"))

(event `self.Deactivate_Hook`
  (bind _staticmesh1 (`self.StaticMesh1`))
  (`GameplayStatics.PlaySoundAtLocation` "/Game/Sounds/Grapnel/metal_ting.metal_ting" (`self.K2_GetActorLocation`))
  (`parent.Deactivate_Hook`)
  (`SceneComponent.K2_SetRelativeRotation` _staticmesh1 (struct :`Roll` -50.0) false false)
  (`PrimitiveComponent.SetMaterial` _staticmesh1 0 "/Game/Meshes/fbx_AssetsMap/GrapActivator/GrapActivatorOFF.GrapActivatorOFF"))

(fn `Toogle`
  (bind _output_get (set `self.Active` (not (`self.Active`))))
  (`PrimitiveComponent.SetMaterial` (`self.Visual`) 0 (select `bool` _output_get :`false` "/Game/Meshes/Materials/PiegesDISABLE.PiegesDISABLE" :`true` "/Game/Meshes/Materials/PiegesACTIVE.PiegesACTIVE" :!type "MaterialInterface Object Reference")))

(fn `UserConstructionScript`
  (`parent.UserConstructionScript`))