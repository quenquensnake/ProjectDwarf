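; Interactable pickup actor that a character can grab and hold, built on a parent interaction Blueprint.
; On Interact it passes itself to the character's PlayerInteractionAC1 component to attempt the pickup.
; ObjectGrabbed turns off collision and physics and matches the mesh rotation to the hand_rSocket on the character mesh.
; ObjectDropped restores collision and physics simulation.
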(event `self.Interact`
  (params (Character :type "/Game/Blueprints/Player_BP Object Reference"))
  (`parent.Interact` Character)
  (bind _interactcharacter (`self.InteractCharacter`)
    (:`then`
      (`/Game/Blueprints/Interaction/PlayerInteraction_AC.AttemptPickup` (`/Game/Blueprints/Player_BP.PlayerInteraction_AC1` _interactcharacter) self))
    (:`else`)))

(event `self.ReceiveBeginPlay`
  (`parent.ReceiveBeginPlay`))

(fn `ObjectDropped`
  (`self.SetActorEnableCollision` self true)
  (`PrimitiveComponent.SetSimulatePhysics` (`self.InteractMesh`) true)
  (`PrimitiveComponent.SetCollisionEnabled` (`self.InteractTrigger`) "QueryAndPhysics")
  (`PrimitiveComponent.SetCollisionEnabled` (`self.InteractMesh`) "QueryAndPhysics"))

(fn `ObjectGrabbed`
  (`self.SetActorEnableCollision` self false)
  (`PrimitiveComponent.SetSimulatePhysics` (`self.InteractMesh`) false)
  (`PrimitiveComponent.SetCollisionEnabled` (`self.InteractTrigger`) "NoCollision")
  (`PrimitiveComponent.SetCollisionEnabled` (`self.InteractMesh`) "NoCollision")
  (`SceneComponent.K2_SetWorldRotation` (`self.InteractMesh`) (`SceneComponent.GetSocketRotation` (`Character.Mesh` (`self.InteractCharacter`)) "hand_rSocket") false false))

(fn `UserConstructionScript`
  (`parent.UserConstructionScript`))