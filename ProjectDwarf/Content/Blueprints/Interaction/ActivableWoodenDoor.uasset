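; Wooden double door that swings open once all of its interruptors are activated, built on a parent activable door class.
; When the parent's toggle event fires with every interruptor active and rotation enabled, a timeline drives RotationDoor on two pivots, negating the alpha on one so they turn in opposite directions.
; The closing trigger event reverses that timeline unless the door is set to MustToggle.
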(event `self.ToggledInterruptors`
  (`parent.ToggledInterruptors`)
  (if (`self.All_Interruptor_Activated`)
    (if (`self.HasToRotate`)
      (bind (_direction _rotating) (`Timeline|Door1_Rotating` :!label _label)
        (:`Update`
          (`self.RotationDoor` _rotating (`self.Pivot1`))
          (`self.RotationDoor` (* _rotating -1.0) (`self.Pivot`)))))))

(event `self.Door_Trigger_Closing`
  (`parent.Door_Trigger_Closing`)
  (if (not (`self.Must_Toggle`))
    (goto _label :!via `Reverse`)))

(fn `UserConstructionScript`
  (`parent.UserConstructionScript`))