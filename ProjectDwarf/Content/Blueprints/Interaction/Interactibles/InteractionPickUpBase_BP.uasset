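; Base Blueprint for interactible objects that a character can pick up and drop.
; On Interact it runs the parent logic, then passes itself to the interacting character's PlayerInteractionAC through AttemptPickup.
; ObjectGrabbed turns off actor collision and mesh physics simulation, and ObjectDropped turns both back on.
; Older per-component collision and socket-rotation nodes remain in the grab and drop functions but never run.
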(event `self.Interact`
  (params (Character :type "/Game/Blueprints/Player_BP Object Reference"))
  (`parent.Interact` Character)
  (bind _interactcharacter (`self.InteractCharacter`)
    (:`then`
      (`/Game/Blueprints/Interaction/Interactibles/PlayerInteraction_AC.AttemptPickup` (`/Game/Blueprints/Player_BP.PlayerInteraction_AC` _interactcharacter) self))
    (:`else`)))

(event `self.ReceiveBeginPlay`
  (`parent.ReceiveBeginPlay`))

(fn `ObjectDropped`
  (`self.SetActorEnableCollision` self true)
  (`PrimitiveComponent.SetSimulatePhysics` (`self.InteractMesh`) true))

(fn `ObjectGrabbed`
  (`self.SetActorEnableCollision` self false)
  (`PrimitiveComponent.SetSimulatePhysics` (`self.InteractMesh`) false))

(fn `UserConstructionScript`
  (`parent.UserConstructionScript`)
  (set `self.RespawnInfo` (`self.RespawnInfo`)))