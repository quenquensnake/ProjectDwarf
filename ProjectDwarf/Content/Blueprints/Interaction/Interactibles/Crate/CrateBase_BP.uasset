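; CrateBase_BP is a crate interactible that can be grabbed and dropped, judging by its path and events, extending behavior from a parent class.
; Its ObjectGrabbed event calls the parent and then disables collision on the whole actor, and ObjectDropped calls the parent and then re-enables it.
; The construction script only calls the parent, and BeginPlay, overlap and Tick are disabled placeholders.
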(event `self.ObjectGrabbed`
  (`parent.ObjectGrabbed`)
  (`self.SetActorEnableCollision` self false))

(event `self.ObjectDropped`
  (`parent.ObjectDropped`)
  (`self.SetActorEnableCollision` self true))

(fn `UserConstructionScript`
  (`parent.UserConstructionScript`))