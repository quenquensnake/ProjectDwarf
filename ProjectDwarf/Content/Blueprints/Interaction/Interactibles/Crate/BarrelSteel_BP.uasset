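; BarrelSteel_BP is an interactible steel barrel that breaks apart when its InteractMesh overlaps an ItemKiller actor.
; The overlap hides the mesh, deactivates the interaction components, enables physics and collision on the Destructible, applies radius damage to fracture it, then destroys the actor after a short delay.
; Tick turns Destructible collision off every frame, including after the break.
; Debug prints and an unconnected alternate break chain remain in the graph.
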(event `self.ReceiveTick`
  (params (DeltaSeconds :type "Float (single-precision)"))
  (`PrimitiveComponent.SetCollisionEnabled` (`self.Destructible`) "NoCollision"))

(event `self.InteractMesh.OnComponentBeginOverlap`
  (params (OverlappedComponent :type "PrimitiveComponent Object Reference") (OtherActor :type "Actor Object Reference") (OtherComp :type "PrimitiveComponent Object Reference") (OtherBodyIndex :type Integer) (bFromSweep :type Boolean) (SweepResult :type "HitResult Structure (by ref)"))
  (bind _destructible (`self.Destructible`))
  (cast `/Game/Blueprints/ItemKiller` OtherActor)
  (`KismetSystemLibrary.PrintString` "PATATE")
  (`SceneComponent.SetVisibility` (`self.InteractMesh`) false false)
  (`ActorComponent.Deactivate` (`self.InteractTrigger`))
  (`ActorComponent.Deactivate` (`self.InteractUI`))
  (`ActorComponent.Deactivate` (`self.TargetComponent`))
  (`PrimitiveComponent.SetCollisionEnabled` _destructible "QueryAndPhysics")
  (`PrimitiveComponent.SetSimulatePhysics` _destructible true)
  (`DestructibleComponent.ApplyRadiusDamage` _destructible 1.0 (`SceneComponent.K2_GetComponentLocation` _destructible) 1.0 1.0 false)
  (`KismetSystemLibrary.Delay` 1.0)
  (`self.K2_DestroyActor`))

(fn `UserConstructionScript`
  (`parent.UserConstructionScript`))