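; InteractionSwitch_BP is an interactible switch that toggles on and off each time a character interacts with it.
; After the parent interaction runs, it flips IsToggledOn and swaps the InteractMesh material between active and disabled looks.
; It also updates the interaction widget prompt to "Turn Off" or "Turn On", when that widget is valid, and calls Activate or Deactivate accordingly.
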(event `self.Interact`
  (params (Character :type "/Game/Blueprints/Player_BP Object Reference"))
  (bind _interactmesh (`self.InteractMesh`))
  (`parent.Interact` Character)
  (if (not (`self.Is_Toggled_On`))
    (set `self.Is_Toggled_On` true)
    (`PrimitiveComponent.SetMaterial` _interactmesh 0 "/Game/Meshes/Materials/PiegesACTIVE.PiegesACTIVE")
    (bind _interactionuiwidget (`self.InteractionUIWidget`)
      (:`then`
        (`/Game/Blueprints/Interaction/Interactibles/InteractionUI_BP.SetInteractDescription` _interactionuiwidget "Turn Off"))
      (:`else`
        _))
    (`self.Activate`)
    (else
      (set `self.Is_Toggled_On` false)
      (`PrimitiveComponent.SetMaterial` _interactmesh 0 "/Game/Meshes/Materials/PiegesDISABLE.PiegesDISABLE")
      (bind _interactionuiwidget_2 (`self.InteractionUIWidget`)
        (:`then`
          (`/Game/Blueprints/Interaction/Interactibles/InteractionUI_BP.SetInteractDescription` _interactionuiwidget_2 "Turn On"))
        (:`else`
          _))
      (`self.Deactivate`))))

(fn `UserConstructionScript`
  (`parent.UserConstructionScript`))