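; Lever_BP is an interactible lever that rotates and changes material according to its toggled state.
; Each Tick plays or reverses the RotationLever timeline based on IsToggledOn, applying its angle as roll combined with the rotation captured at BeginPlay.
; Interact calls the parent logic, then sets the Base mesh to the active or disabled material to match IsToggledOn.
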(event `self.ReceiveBeginPlay`
  (`parent.ReceiveBeginPlay`)
  (set `self.StartRotation` (`SceneComponent.K2_GetComponentRotation` (`self.Base`))))

(event `self.ReceiveTick`
  (params (DeltaSeconds :type "Float (single-precision)"))
  (if (`self.Is_Toggled_On`)
    (bind (_direction _angle) (`Timeline|RotationLever` :!label _label)
      (:`Update`
        (`SceneComponent.K2_SetWorldRotation` (`self.Base`) (`KismetMathLibrary.ComposeRotators` (`KismetMathLibrary.MakeRotator` _angle) (`self.StartRotation`)) false false)))
    (else
      (goto _label :!via `Reverse`))))

(event `self.Interact`
  (params (Character :type "/Game/Blueprints/Player_BP Object Reference"))
  (bind _base (`self.Base`))
  (`parent.Interact` Character)
  (if (`self.Is_Toggled_On`)
    (`PrimitiveComponent.SetMaterial` _base 0 "/Game/Meshes/Materials/PiegesACTIVE.PiegesACTIVE")
    (else
      (`PrimitiveComponent.SetMaterial` _base 0 "/Game/Meshes/Materials/PiegesDISABLE.PiegesDISABLE"))))

(fn `UserConstructionScript`
  (`parent.UserConstructionScript`))