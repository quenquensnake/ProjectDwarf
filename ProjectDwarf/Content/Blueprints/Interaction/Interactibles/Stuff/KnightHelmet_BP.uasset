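; Grabbable knight helmet interactible that sockets onto a knight AI and can be taken from it.
; AttachToKnight snaps it to the helmet socket and disables physics and interaction, while DetachFromKnight drops it as a physics object.
; Stun and DeStun toggle whether it can be targeted and grabbed.
; Attaching, detaching and grabbing update the knight's head flag, helmet material and BlueFlames emitter, which burns while the helmet is off.
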(event `self.ObjectGrabbed`
  (`parent.ObjectGrabbed`)
  (set `/Game/Blueprints/AI/AI_BP/AI_BP.HeadOnKnightAI` false (`self.KnightRef`))
  (`PrimitiveComponent.SetMaterial` (`self.InteractMesh`) 0 "/Game/Meshes/fbx_Knight/Textures/HelmetDesactivated/HeadDesactivated.HeadDesactivated")
  (`ParticleSystemComponent.SetEmitterEnable` (`/Game/Blueprints/AI/AI_BP/AI_BP.ParticleSystem` (`self.KnightRef`)) "BlueFlames" true))

(fn `AttachToKnight`
  (params (Knight :type "/Game/Blueprints/AI/AI_BP/AI_BP Object Reference"))
  (bind _interactmesh (`self.InteractMesh`))
  (bind _output_get (set `self.KnightRef` Knight))
  (set `/Game/Blueprints/AI/AI_BP/AI_BP.HeadOnKnightAI` true _output_get)
  (`PrimitiveComponent.SetMaterial` _interactmesh 0 "/Game/Meshes/fbx_Knight/Textures/Knight_material.Knight_material")
  (`PrimitiveComponent.SetSimulatePhysics` _interactmesh false)
  (`PrimitiveComponent.SetCollisionEnabled` _interactmesh "QueryOnly")
  (`PrimitiveComponent.SetCollisionEnabled` (`self.InteractTrigger`) "NoCollision")
  (set `/Game/Blueprints/Graplin/TargetComponent.isAvailable` false (`self.TargetComponent`))
  (set `self.IsTake` false)
  (`self.K2_AttachToComponent` (`Character.Mesh` Knight) "KnightHelmetSocket" "SnapToTarget" "SnapToTarget" "SnapToTarget")
  (`ParticleSystemComponent.SetEmitterEnable` (`/Game/Blueprints/AI/AI_BP/AI_BP.ParticleSystem` (`self.KnightRef`)) "BlueFlames" false))

(fn `DeStun`
  (`PrimitiveComponent.SetCollisionEnabled` (`self.InteractTrigger`) "NoCollision")
  (set `/Game/Blueprints/Graplin/TargetComponent.isAvailable` false (`self.TargetComponent`)))

(fn `DetachFromKnight`
  (bind _interactmesh (`self.InteractMesh`))
  (set `/Game/Blueprints/AI/AI_BP/AI_BP.HeadOnKnightAI` false (`self.KnightRef`))
  (`self.K2_DetachFromActor` "KeepWorld" "KeepWorld" "KeepWorld")
  (`PrimitiveComponent.SetMaterial` _interactmesh 0 "/Game/Meshes/fbx_Knight/Textures/HelmetDesactivated/HeadDesactivated.HeadDesactivated")
  (`PrimitiveComponent.SetCollisionEnabled` _interactmesh "QueryAndPhysics")
  (`PrimitiveComponent.SetSimulatePhysics` _interactmesh true)
  (`ParticleSystemComponent.SetEmitterEnable` (`/Game/Blueprints/AI/AI_BP/AI_BP.ParticleSystem` (`self.KnightRef`)) "BlueFlames" true))

(fn `Stun`
  (`PrimitiveComponent.SetCollisionEnabled` (`self.InteractTrigger`) "QueryOnly")
  (set `/Game/Blueprints/Graplin/TargetComponent.isAvailable` true (`self.TargetComponent`)))

(fn `UserConstructionScript`
  (`parent.UserConstructionScript`))