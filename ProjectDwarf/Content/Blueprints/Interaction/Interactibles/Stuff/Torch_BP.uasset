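; Torch actor with a flickering light that can light campfires on contact.
; BeginPlay runs an endless Delay loop that sets TorchLight to a random intensity at short random intervals to mimic a flame.
; When the FireCollision component begins overlapping a CampFire, it calls that actor's ActiveFire.
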(event `self.ReceiveBeginPlay`
  (`parent.ReceiveBeginPlay`)
  ;[1 1 1] Light Flick
  (`LightComponent.SetIntensity` (`self.TorchLight`) (`KismetMathLibrary.RandomFloatInRange` 15000.0 19000.0) :!label _label)
  (`KismetSystemLibrary.Delay` (`KismetMathLibrary.RandomFloatInRange` 0.0 0.2))
  (goto _label))

(event `self.FireCollision.OnComponentBeginOverlap`
  (params (OverlappedComponent :type "PrimitiveComponent Object Reference") (OtherActor :type "Actor Object Reference") (OtherComp :type "PrimitiveComponent Object Reference") (OtherBodyIndex :type Integer) (bFromSweep :type Boolean) (SweepResult :type "HitResult Structure (by ref)"))
  (bind _ascamp_fire (cast `/Game/Blueprints/CampFire` OtherActor))
  (`/Game/Blueprints/CampFire.ActiveFire` _ascamp_fire))

(fn `UserConstructionScript`
  (`parent.UserConstructionScript`))