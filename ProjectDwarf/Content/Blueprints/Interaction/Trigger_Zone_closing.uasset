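; Trigger zone that closes its associated door once both players have passed through it.
; The main box flags each player by Id and counts them; at two, it clears the door's MustToggle and calls DoorClosing.
; Entering the security box clears that player's flag and decrements the count.
; The door is resolved by chained casts to wooden, standard or big activable door classes.
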(event `self.ReceiveBeginPlay`
  (set `self.P1 has passed` false)
  (set `self.P2 has passed` false)
  (set `self.Actors Numbers` 0))

(event `self.Box.OnComponentBeginOverlap`
  (params (OverlappedComponent :type "PrimitiveComponent Object Reference") (OtherActor :type "Actor Object Reference") (OtherComp :type "PrimitiveComponent Object Reference") (OtherBodyIndex :type Integer) (bFromSweep :type Boolean) (SweepResult :type "HitResult Structure (by ref)"))
  (bind _actors_numbers (`self.Actors Numbers`))
  (bind _associated_door (`self.Associated_Door`))
  (bind _asplayer_bp (cast `/Game/Blueprints/Player_BP` OtherActor))
  (if (== (`/Game/Blueprints/Player_BP.Id` _asplayer_bp) 0)
    (if (not (`self.P1 has passed`))
      (set `self.P1 has passed` true)
      (`/Engine/EditorBlueprintResources/StandardMacros.IncrementInt` _actors_numbers :!label _label
        (:`  `
          (if (>= _actors_numbers 2)
            (bind _asactivable_wooden_door (cast `/Game/Blueprints/Interaction/ActivableWoodenDoor` _associated_door)
              (:`then`
                (set `/Game/Blueprints/Interaction/ActivableDoor.Must_Toggle` false _asactivable_wooden_door)
                (`/Game/Blueprints/Interaction/ActivableDoor.DoorClosing` _asactivable_wooden_door))
              (:`CastFailed`
                (bind _asactivable_door (cast `/Game/Blueprints/Interaction/ActivableDoor` _associated_door)
                  (:`then`
                    (set `/Game/Blueprints/Interaction/ActivableDoor.Must_Toggle` false _asactivable_door)
                    (`/Game/Blueprints/Interaction/ActivableDoor.DoorClosing` _asactivable_door))
                  (:`CastFailed`
                    (bind _asactivable_big_door (cast `/Game/Blueprints/Interaction/ActivableBigDoor` _associated_door))
                    (set `/Game/Blueprints/Interaction/ActivableDoor.Must_Toggle` false _asactivable_big_door)
                    (`/Game/Blueprints/Interaction/ActivableDoor.DoorClosing` _asactivable_big_door)))))))))
    (elif (not (`self.P2 has passed`))
      (set `self.P2 has passed` true)
      (goto _label))))

(event `self.security_box.OnComponentBeginOverlap`
  (params (OverlappedComponent :type "PrimitiveComponent Object Reference") (OtherActor :type "Actor Object Reference") (OtherComp :type "PrimitiveComponent Object Reference") (OtherBodyIndex :type Integer) (bFromSweep :type Boolean) (SweepResult :type "HitResult Structure (by ref)"))
  (bind _asplayer_bp (cast `/Game/Blueprints/Player_BP` OtherActor))
  (if (== (`/Game/Blueprints/Player_BP.Id` _asplayer_bp) 0)
    (if (`self.P1 has passed`)
      (set `self.P1 has passed` false)
      (`/Engine/EditorBlueprintResources/StandardMacros.DecrementInt` (`self.Actors Numbers`) :!label _label_2))
    (elif (`self.P2 has passed`)
      (set `self.P2 has passed` false)
      (goto _label_2))))

(event `self.security_box.OnComponentEndOverlap`
  (params (OverlappedComponent :type "PrimitiveComponent Object Reference") (OtherActor :type "Actor Object Reference") (OtherComp :type "PrimitiveComponent Object Reference") (OtherBodyIndex :type Integer)))

(fn `UserConstructionScript`)