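; Interaction_BP is an interactable actor with a mesh, sphere trigger and widget prompt.
; The construction script configures these components from variables, and BeginPlay passes the interaction description to the InteractionUI_BP widget.
; Trigger overlaps add or remove the actor on the Player_BP's PlayerInteraction_AC component.
; It exposes ToggleUI for prompt visibility and a placeholder Interact that only stores the character and prints a message.
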(event `self.ReceiveBeginPlay`
  (bind _asinteraction_ui_bp (cast `/Game/Blueprints/Interaction/InteractionUI_BP` (`WidgetComponent.GetUserWidgetObject` (`self.InteractUI`))))
  (bind _output_get (set `self.InteractionUIWidget` _asinteraction_ui_bp))
  (`/Game/Blueprints/Interaction/InteractionUI_BP.SetInteractDescription` _output_get (`self.InteractDescription`)))

(event `self.InteractTrigger.OnComponentBeginOverlap`
  (params (OverlappedComponent :type "PrimitiveComponent Object Reference") (OtherActor :type "Actor Object Reference") (OtherComp :type "PrimitiveComponent Object Reference") (OtherBodyIndex :type Integer) (bFromSweep :type Boolean) (SweepResult :type "HitResult Structure (by ref)"))
  ;[1 1 1] Trigger Overlap
  (bind _asplayer_bp (cast `/Game/Blueprints/Player_BP` OtherActor))
  (bind _returnvalue (`self.GetComponentByClass` _asplayer_bp "/Game/Blueprints/Interaction/PlayerInteraction_AC.PlayerInteraction_AC_C"))
  (`/Engine/EditorBlueprintResources/StandardMacros.IsValid` _returnvalue
    (:`Is Valid`
      (`/Game/Blueprints/Interaction/PlayerInteraction_AC.AddInteraction` _returnvalue self))))

(event `self.InteractTrigger.OnComponentEndOverlap`
  (params (OverlappedComponent :type "PrimitiveComponent Object Reference") (OtherActor :type "Actor Object Reference") (OtherComp :type "PrimitiveComponent Object Reference") (OtherBodyIndex :type Integer))
  ;[1 1 1] Trigger Overlap
  (bind _asplayer_bp (cast `/Game/Blueprints/Player_BP` OtherActor))
  (bind _returnvalue (`self.GetComponentByClass` _asplayer_bp "/Game/Blueprints/Interaction/PlayerInteraction_AC.PlayerInteraction_AC_C"))
  (`/Engine/EditorBlueprintResources/StandardMacros.IsValid` _returnvalue
    (:`Is Valid`
      (`/Game/Blueprints/Interaction/PlayerInteraction_AC.RemoveInteraction` _returnvalue self))))

(fn `Interact`
  (params (Character :type "/Game/Blueprints/Player_BP Object Reference"))
  (set `self.InteractCharacter` Character)
  (`KismetSystemLibrary.PrintString` "INTERACTED"))

(fn `SetupMesh`
  (`StaticMeshComponent.SetStaticMesh` (`self.InteractMesh`) (`self.InteractionMesh`))
  (`SceneComponent.K2_SetRelativeTransform` (`self.InteractMesh`) (`self.MeshTransform`) false false))

(fn `SetupTrigger`
  (`SphereComponent.SetSphereRadius` (`self.InteractTrigger`) (`self.TriggerRadius`) true)
  (`SceneComponent.K2_SetRelativeLocation` (`self.InteractTrigger`) (`self.TriggerLocation`) false false))

(fn `SetupUI`
  (`SceneComponent.K2_SetRelativeLocation` (`self.InteractUI`) (`self.UILocation`) false false))

(fn `ToggleUI`
  (params (bVisible :type Boolean))
  (`SceneComponent.SetVisibility` (`self.InteractUI`) bVisible false))

(fn `UserConstructionScript`
  (`self.SetupMesh`)
  (`self.SetupTrigger`)
  (`self.SetupUI`))