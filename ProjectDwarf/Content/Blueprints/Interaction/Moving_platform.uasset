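; Moving platform that travels between its start location and an editable offset, either on its own or driven by levers.
; Timelines lerp its position, with play rate derived from speed over distance, and ping-pong with pauses when self-moving.
; Otherwise it binds to lever activate/deactivate events, advancing once all switches and interruptors are on and reversing if not.
; Toggle mode switches it to self-moving instead.
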(event `PlatformStart`
  (`self.Platform_Trigger_Move`))

(event `PlatformEnd`
  (`self.Platform_Trigger_Closing`))

(event `self.ReceiveBeginPlay`
  (bind _returnvalue (/ (`self.speed_edited`) (`KismetMathLibrary.VSize` (- (`self.Plaform_Starting_Location`) (`self.Platform_End_Location`)))))
  ;[1 1 1] Custom platform Offset and speed
  (bind _output_get (set `self.Plaform_Starting_Location` (`SceneComponent.RelativeLocation` (`self.moving_platform`))))
  (set `self.Platform_End_Location` (+ _output_get (`self.Platform_Offset`)))
  (`TimelineComponent.SetPlayRate` (`self.Movement`) _returnvalue)
  (`TimelineComponent.SetPlayRate` (`self.Reverse_Movement`) _returnvalue)
  (if (`self.Move_on_its_Own`)
    ;[1 1 1] Moving platform
    (bind (_direction _reverse_moving) (`Timeline|Movement` :!via `PlayFromStart` :!label _label)
      (:`Update`
        (`SceneComponent.K2_SetRelativeLocation` (`self.moving_platform`) (`KismetMathLibrary.VLerp` (`self.Plaform_Starting_Location`) (`self.Platform_End_Location`) _reverse_moving) false false))
      (:`Finished`
        (if (`self.Move_on_its_Own`)
          (`KismetSystemLibrary.Delay` 1.0)
          ;[1 1 1] Revert Moving platform
          (bind (_direction_2 _moving) (`Timeline|Reverse_Movement` :!via `PlayFromStart`)
            (:`Update`
              (`SceneComponent.K2_SetRelativeLocation` (`self.moving_platform`) (`KismetMathLibrary.VLerp` (`self.Platform_End_Location`) (`self.Plaform_Starting_Location`) _moving) false false))
            (:`Finished`
              (`KismetSystemLibrary.Delay` 1.0)
              (goto _label :!via `PlayFromStart`))))))
    (else
      (for _array_element (`self.tab_switches`)
        (bind _aslever_bp (cast `/Game/Blueprints/Interaction/Interactibles/Lever_BP` _array_element))
        (add `/Game/Blueprints/Interaction/Interactibles/InteractionSwitch_BP.Activate` _aslever_bp (delegate `PlatformStart`))
        (add `/Game/Blueprints/Interaction/Interactibles/InteractionSwitch_BP.Deactivate` _aslever_bp (delegate `PlatformEnd`))))))

(event `Platform_Trigger_Move`
  ;[1 1 1] Check if each interruptors is toggled
  (if (not (`self.Move_on_its_Own`))
    (set `self.All_Interruptor_Activated` true)
    (for _array_element (`self.tab_interrupt`)
      (if (not (`/Game/Blueprints/Interaction/Moving_platform_Pressure_plate_BP.Is_Toggled_On` _array_element))
        (set `self.All_Interruptor_Activated` false)))
    (for _array_element_2 (`self.tab_switches`)
      (if (not (`/Game/Blueprints/Interaction/Interactibles/InteractionSwitch_BP.Is_Toggled_On` _array_element_2))
        (set `self.All_Interruptor_Activated` false)))
    (if (`self.All_Interruptor_Activated`)
      (if (`self.Is_Toggled_On`)
        (set `self.Move_on_its_Own` true)
        (goto _label :!via `PlayFromStart`)
        (else
          (goto _label)))
      (else
        (goto _label :!via `Reverse`)))))

(event `Platform_Trigger_Closing`
  ;[1 1 1] Close the platform depending if Toggle Mode is On/Off
  (if (`self.Is_Toggled_On`)
    (set `self.Move_on_its_Own` true)
    (else
      (goto _label :!via `Reverse`))))

(fn `UserConstructionScript`)