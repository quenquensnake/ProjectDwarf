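; Pressure plate that opens a linked Door when weighed down and closes it when released.
; Trigger overlaps count untagged components meeting RequiredWeight; a special flag rejects pickups other than steel barrels.
; Pickup drop events also decrement the count, while hookable plates skip weight checks and use Activate/Deactivate_Hook events.
; Toggling plays slab sounds and drives a timeline that moves the plate visual and swaps its material.
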(event `self.ReceiveBeginPlay`
  ;[1 1 1] Start
  (set `self.Required_Weight` 20.0)
  (set `self.Interruptor_Offset` (0.0 0.0 -6.0)))

(event `self.TriggerZone.OnComponentEndOverlap`
  (params (OverlappedComponent :type "PrimitiveComponent Object Reference") (OtherActor :type "Actor Object Reference") (OtherComp :type "PrimitiveComponent Object Reference") (OtherBodyIndex :type Integer))
  (bind _visual (`self.Visual`))
  ;[1 1 1] Check leaving trigger conditions
  (if (`ActorComponent.ComponentHasTag` OtherComp "DoesntTriggerPlate")
    _
    (elif (`self.Is_Hookable`)
      _
      (elif (>= (`PrimitiveComponent.GetMass` OtherComp) (`self.Required_Weight`))
        (bind _result (`/Engine/EditorBlueprintResources/StandardMacros.DecrementInt` (`self.Actors_Number`) :!label _label)
          (:`  `
            (if (<= _result 0)
              (set `self.Is_Toggled_On` false :!label _label_2)
              (`/Game/Blueprints/Interaction/ActivableDoor.Door_Trigger_Closing` (`self.Door`))
              ;[1 1 1] Sound Play or Stop
              (`GameplayStatics.SpawnSound2D` "/Game/Sounds/Interactibles/stone_slab_pull.stone_slab_pull" 1.0 1.0 0.0 "/Game/Blueprints/Interaction/Sound_Concurrency.Sound_Concurrency" false false)
              ;[1 1 1] Move Interruptor
              (bind (_direction _lerp) (`Timeline|Interruptor_push` :!via `Reverse` :!label _label_3)
                (:`Update`
                  (`PrimitiveComponent.SetMaterial` _visual 0 (select `bool` (`self.Is_Toggled_On`) :`false` "/Game/StarterContent/Materials/M_Rock_Slate.M_Rock_Slate" :`true` "/Game/Meshes/Materials/PiegesACTIVE.PiegesACTIVE" :!type "MaterialInterface Object Reference"))
                  (`SceneComponent.K2_SetRelativeLocation` _visual (`KismetMathLibrary.VLerp` (* (0.0 0.0 0.0) 1.0) (`self.Interruptor_Offset`) _lerp) false false))))))))))

(event `self.ReceiveTick`
  (params (DeltaSeconds :type "Float (single-precision)"))
  (if (`PrimitiveComponent.IsOverlappingActor` (`self.TriggerZone`) null)
    _))

(event `Deactivate_Hook`
  ;[1 1 1] Check leaving trigger conditions
  (goto _label_2))

(event `self.TriggerZone.OnComponentBeginOverlap`
  (params (OverlappedComponent :type "PrimitiveComponent Object Reference") (OtherActor :type "Actor Object Reference") (OtherComp :type "PrimitiveComponent Object Reference") (OtherBodyIndex :type Integer) (bFromSweep :type Boolean) (SweepResult :type "HitResult Structure (by ref)"))
  ;[1 1 1] Check mass of triggering object
  (bind _asinteraction_pick_up_base_bp (cast `/Game/Blueprints/Interaction/Interactibles/InteractionPickUpBase_BP` OtherActor)
    (:`then`
      (if (`self.MyParentsTellMeImSpecial`)
        (bind _asbarrel_steel_bp (cast `/Game/Blueprints/Interaction/Interactibles/Crate/BarrelSteel_BP` OtherActor)))
      (add `/Game/Blueprints/Interaction/Interactibles/InteractionPickUpBase_BP.Drop` _asinteraction_pick_up_base_bp (delegate `Leaving plate`))
      (add `/Game/Blueprints/Interaction/Interactibles/InteractionPickUpBase_BP.Drop` _asbarrel_steel_bp (delegate `Leaving plate`)))
    (:`CastFailed`
      _))
  (if (`self.Is_Hookable`)
    _
    (elif (`ActorComponent.ComponentHasTag` OtherComp "DoesntTriggerPlate")
      _
      (elif (>= (`PrimitiveComponent.GetMass` OtherComp) (`self.Required_Weight`))
        (`/Engine/EditorBlueprintResources/StandardMacros.IncrementInt` (`self.Actors_Number`)
          (:`  `
            (set `self.Is_Toggled_On` true :!label _label_4)
            (`/Game/Blueprints/Interaction/ActivableDoor.Door_Trigger_Opening` (`self.Door`))
            ;[1 1 1] Sound Play or Stop
            (`GameplayStatics.SpawnSound2D` "/Game/Sounds/Interactibles/stone_slab_push.stone_slab_push" 1.0 1.0 0.0 "/Game/Blueprints/Interaction/Sound_Concurrency.Sound_Concurrency" false false)
            (goto _label_3)))))))

(event `Activate_Hook`
  ;[1 1 1] Check mass of triggering object
  (goto _label_4))

(event `Leaving plate`
  ;[1 1 1] Check mass of triggering object
  (goto _label))

(fn `UserConstructionScript`)