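; Player interaction component that picks which nearby registered interaction the player is targeting and shows its UI.
; Interactions are added to or removed from a list, which unpauses or pauses a looping timer used instead of Tick.
; Each update scores entries by dot product of owner forward and direction to their UI, selecting the highest above a threshold.
; Selection clears while the owner is falling or none qualifies.
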(event `self.ReceiveBeginPlay`
  (bind _returnvalue (`KismetSystemLibrary.K2_SetTimer` null "UpdateInteraction" (`self.InteractionUpdateRate`) true))
  (bind _output_get (set `self.InteractionTimer` _returnvalue))
  (`KismetSystemLibrary.K2_PauseTimerHandle` _output_get))

(fn `AddInteraction`
  (params (Interaction :type "/Game/Blueprints/Interaction_BP Object Reference"))
  (bind _interactionlist (`self.InteractionList`))
  (bind _interactiontimer (`self.InteractionTimer`))
  (`KismetArrayLibrary.Array_AddUnique` _interactionlist Interaction)
  (if (> (`KismetArrayLibrary.Array_Length` _interactionlist) 0)
    (`KismetSystemLibrary.K2_UnPauseTimerHandle` _interactiontimer)
    (else
      (`KismetSystemLibrary.K2_PauseTimerHandle` _interactiontimer)
      (`self.SetBestInteraction` null))))

(fn `GetBestInteraction`
  (locals (Dots :type "Array of Float (double-precision)"))
  (bind _returnvalue (`self.GetOwner`))
  (bind (_indexofmaxvalue _maxvalue) (`KismetMathLibrary.MaxOfFloatArray` (`local.Dots`)))
  (for _array_element (`self.InteractionList`)
    (`KismetArrayLibrary.Array_Add` (`local.Dots`) (`KismetMathLibrary.Dot_VectorVector` (`KismetMathLibrary.Normal` (- (`SceneComponent.K2_GetComponentLocation` (`/Game/Blueprints/Interaction_BP.InteractUI` _array_element)) (`Actor.K2_GetActorLocation` _returnvalue))) (`Actor.GetActorForwardVector` _returnvalue))))
  (if (>= _maxvalue (`self.InteractThreshold`))
    (`self.SetBestInteraction` (`|GetArrayItem` (`self.InteractionList`) _indexofmaxvalue))
    (else
      (`self.SetBestInteraction` null))))

(fn `RemoveInteraction`
  (params (Interaction :type "/Game/Blueprints/Interaction_BP Object Reference"))
  (bind _interactionlist (`self.InteractionList`))
  (bind _interactiontimer (`self.InteractionTimer`))
  (`KismetArrayLibrary.Array_RemoveItem` _interactionlist Interaction)
  (if (> (`KismetArrayLibrary.Array_Length` _interactionlist) 0)
    (`KismetSystemLibrary.K2_UnPauseTimerHandle` _interactiontimer)
    (else
      (`KismetSystemLibrary.K2_PauseTimerHandle` _interactiontimer)
      (`self.SetBestInteraction` null))))

(fn `SetBestInteraction`
  (params (Interaction :type "/Game/Blueprints/Interaction_BP Object Reference"))
  (locals (NewInteraction :type "/Game/Blueprints/Interaction_BP Object Reference"))
  (bind _output_get (set `local.NewInteraction` Interaction))
  (`/Engine/EditorBlueprintResources/StandardMacros.IsValid` _output_get
    (:`Is Valid`
      (if (!= (`local.NewInteraction`) (`self.SelectedInteraction`))
        (bind _selectedinteraction (`self.SelectedInteraction`)
          (:`then`
            (`/Game/Blueprints/Interaction_BP.ToggleUI` _selectedinteraction false))
          (:`else`
            _))
        (bind _output_get_2 (set `self.SelectedInteraction` (`local.NewInteraction`)))
        (`/Game/Blueprints/Interaction_BP.ToggleUI` _output_get_2 true)))
    (:`Is Not Valid`
      (bind _selectedinteraction_2 (`self.SelectedInteraction`)
        (:`then`
          (`/Game/Blueprints/Interaction_BP.ToggleUI` _selectedinteraction_2 false)
          (set `self.SelectedInteraction` null))
        (:`else`)))))

(fn `ShouldUpdateInteraction`
  (returns (ShouldUpdate :type Boolean))
  (return (and (> (`KismetArrayLibrary.Array_Length` (`self.InteractionList`)) 0) (not (`NavMovementComponent.IsFalling` (`Actor.GetComponentByClass` (`self.GetOwner`) "/Script/Engine.CharacterMovementComponent"))))))

(fn `UpdateInteraction`
  (bind _shouldupdate (`self.ShouldUpdateInteraction`))
  (if _shouldupdate
    (`self.GetBestInteraction`)
    (else
      (`self.SetBestInteraction` null))))