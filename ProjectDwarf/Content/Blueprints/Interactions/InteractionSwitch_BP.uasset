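; Toggle switch interactable that alternates between on and off each time a character interacts with it.
; Interact runs the parent logic, then flips the Active flag and swaps the mesh material between gold metal and basic wall.
; It updates the interaction widget prompt to "Turn Off" or "Turn On" when the widget is valid, then calls the Activate or Deactivate dispatcher.
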(event `self.Interact`
  (params (Character :type "/Game/Blueprints/Player_BP Object Reference"))
  (bind _interactmesh (`self.InteractMesh`))
  (`parent.Interact` Character)
  (if (not (`self.bActive`))
    (set `self.bActive` true)
    (`PrimitiveComponent.SetMaterial` _interactmesh 0 "/Game/StarterContent/Materials/M_Metal_Gold.M_Metal_Gold")
    (bind _interactionuiwidget (`self.InteractionUIWidget`)
      (:`then`
        (`/Game/Blueprints/InteractionUI_BP.SetInteractDescription` _interactionuiwidget "Turn Off"))
      (:`else`
        _))
    (`self.Activate`)
    (else
      (set `self.bActive` false)
      (`PrimitiveComponent.SetMaterial` _interactmesh 0 "/Game/StarterContent/Materials/M_Basic_Wall.M_Basic_Wall")
      (bind _interactionuiwidget_2 (`self.InteractionUIWidget`)
        (:`then`
          (`/Game/Blueprints/InteractionUI_BP.SetInteractDescription` _interactionuiwidget_2 "Turn On"))
        (:`else`
          _))
      (`self.Deactivate`))))

(fn `UserConstructionScript`
  (`parent.UserConstructionScript`))