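; Axe_BP is a melee weapon Blueprint that damages whatever lies in front of the player when its Attack event fires.
; Attack sphere-traces on the Camera channel from the player along their forward vector to WeaponRange, ignoring the player, and applies damage to each hit actor.
; The owner cast that would set PlayerBPRef and the explosion effect and sound nodes are disconnected, so none run.
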(event `self.ReceiveBeginPlay`)

(event `Attack`
  (bind _playerbp_ref (`self.PlayerBP_Ref`))
  (bind _returnvalue (`self.K2_GetActorLocation` _playerbp_ref))
  (bind (_outhits _returnvalue_2) (`KismetSystemLibrary.SphereTraceMulti` _returnvalue (+ _returnvalue (* (`self.GetActorForwardVector` _playerbp_ref) (`self.WeaponRange`))) 25.0 "TraceTypeQuery2" false (`|MakeArray` _playerbp_ref :!type "Actor Object Reference")))
  (if _returnvalue_2
    (for _array_element _outhits
      (`GameplayStatics.ApplyDamage` (`.HitActor` (`GameplayStatics.BreakHitResult` _array_element)) 1.0 null (`self.PlayerBP_Ref`)))))

(fn `UserConstructionScript`)