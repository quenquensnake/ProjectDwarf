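; Launcher projectile actor that knocks the player away on impact.
; LaunchProjectile sets a local-space forward velocity on ProjectileMovement at the given speed and returns that vector.
; On hitting a Player_BP, it enables capsule physics and applies a large impulse along world +X, regardless of projectile facing.
; One second after any hit it destroys itself, first setting CapsuleHasHit if the target was the player.
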(event `self.CollisionMesh.OnComponentHit`
  (params (HitComponent :type "PrimitiveComponent Object Reference") (OtherActor :type "Actor Object Reference") (OtherComp :type "PrimitiveComponent Object Reference") (NormalImpulse :type "Vector Structure") (Hit :type "HitResult Structure (by ref)"))
  (bind _asplayer_bp (cast `/Game/Blueprints/Player_BP` OtherActor)
    (:`then`
      (bind _capsulecomponent (`Character.CapsuleComponent` _asplayer_bp))
      (`PrimitiveComponent.SetSimulatePhysics` _capsulecomponent true)
      (`PrimitiveComponent.AddImpulse` _capsulecomponent (* (`KismetMathLibrary.GetForwardVector` (struct)) 150000.0) "None" false)
      (`KismetSystemLibrary.Delay` 1.0)
      (set `/Game/Blueprints/Player_BP.CapsuleHasHit` true _asplayer_bp)
      (`self.K2_DestroyActor`))
    (:`CastFailed`
      (`KismetSystemLibrary.Delay` 1.0)
      (`self.K2_DestroyActor`))))

(fn `LaunchProjectile`
  (params (Speed :type "Float (double-precision)"))
  (returns (LaunchVelocity :type "Vector Structure"))
  (bind _returnvalue (* (`KismetMathLibrary.GetForwardVector` (struct)) Speed))
  (`ProjectileMovementComponent.SetVelocityInLocalSpace` (`self.ProjectileMovement`) _returnvalue)
  (return _returnvalue))

(fn `UserConstructionScript`)