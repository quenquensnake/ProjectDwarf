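; Projectile launcher actor that automatically fires arrows on a repeating timer.
; BeginPlay starts a looping timer at the LaunchTimer interval, which calls Fire.
; Fire spawns an Arrow at the static mesh's FireSocket transform and calls its LaunchProjectile with LaunchSpeed.
; A debug trajectory prediction using the returned launch velocity is present but disconnected, so it never runs.
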(event `self.ReceiveBeginPlay`
  (`KismetSystemLibrary.K2_SetTimer` null "Fire" (`self.LaunchTimer`) true))

(fn `Fire`
  (bind _returnvalue (`|SpawnActorFromClass` "/Game/Blueprints/Launcher/Arrow.Arrow_C" (`SceneComponent.GetSocketTransform` (`self.StaticMesh`) "FireSocket" "RTS_World") "Undefined" "OverrideRootScale"))
  (bind _launchvelocity (`/Game/Blueprints/Launcher/Arrow.LaunchProjectile` _returnvalue (`self.LaunchSpeed`))))

(fn `UserConstructionScript`)