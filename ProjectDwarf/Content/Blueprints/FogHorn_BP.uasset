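; FogHorn_BP is a fog horn actor that pushes whatever overlaps its Box volume along the actor's forward vector.
; Every Tick it applies a fixed, mass-dependent impulse to each overlapping actor's primitive root component, so the push scales with frame rate.
; The construction script resets the Arrow's world scale to one, keeping it unaffected by actor scaling.
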(event `self.ReceiveTick`
  (params (DeltaSeconds :type "Float (single-precision)"))
  (for _array_element (`PrimitiveComponent.GetOverlappingActors` (`self.Box`) null)
    (bind _asprimitive_component (cast `PrimitiveComponent` (`self.K2_GetRootComponent` _array_element)))
    (`PrimitiveComponent.AddImpulse` _asprimitive_component (* (`self.GetActorForwardVector`) 2000.0) "None" false)))

(fn `UserConstructionScript`
  (`SceneComponent.SetWorldScale3D` (`self.Arrow`) (1.0 1.0 1.0)))