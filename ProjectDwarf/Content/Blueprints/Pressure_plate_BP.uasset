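; Pressure plate that opens a linked Door while sufficiently heavy objects rest on its TriggerZone.
; Overlapping components at or above RequiredWeight raise a counter and trigger door opening; lighter ones only print a message.
; When the last heavy object leaves, the door closes.
; The Interruptor_push timeline plays forward or in reverse to lerp the plate's Visual between rest and pressed offset.
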(event `self.ReceiveBeginPlay`
  ;[1 1 1] Start
  (set `self.Required_Weight` 20.0)
  (set `self.Interruptor_Offset` (0.0 0.0 -8.0)))

(event `self.TriggerZone.OnComponentEndOverlap`
  (params (OverlappedComponent :type "PrimitiveComponent Object Reference") (OtherActor :type "Actor Object Reference") (OtherComp :type "PrimitiveComponent Object Reference") (OtherBodyIndex :type Integer))
  ;[1 1 1] Check leaving trigger conditions
  (if (>= (`PrimitiveComponent.GetMass` OtherComp) (`self.Required_Weight`))
    (bind _result (`/Engine/EditorBlueprintResources/StandardMacros.DecrementInt` (`self.Actors_Number`))
      (:`  `
        (if (<= _result 0)
          (set `self.Is_Toggled_On` false)
          (`/Game/Blueprints/ActivableDoor.Door_Trigger_Closing` (`self.Door`))
          ;[1 1 1] Move Interruptor
          (bind (_direction _lerp) (`Timeline|Interruptor_push` :!via `Reverse` :!label _label)
            (:`Update`
              (`SceneComponent.K2_SetRelativeLocation` (`self.Visual`) (`KismetMathLibrary.VLerp` (* (0.0 0.0 0.0) 1.0) (`self.Interruptor_Offset`) _lerp) false false))))))))

(event `self.TriggerZone.OnComponentBeginOverlap`
  (params (OverlappedComponent :type "PrimitiveComponent Object Reference") (OtherActor :type "Actor Object Reference") (OtherComp :type "PrimitiveComponent Object Reference") (OtherBodyIndex :type Integer) (bFromSweep :type Boolean) (SweepResult :type "HitResult Structure (by ref)"))
  ;[1 1 1] Check mass of triggering object
  (if (>= (`PrimitiveComponent.GetMass` OtherComp) (`self.Required_Weight`))
    (`/Engine/EditorBlueprintResources/StandardMacros.IncrementInt` (`self.Actors_Number`)
      (:`  `
        (set `self.Is_Toggled_On` true)
        (`/Game/Blueprints/ActivableDoor.Door_Trigger_Opening` (`self.Door`))
        (goto _label)))
    (else
      (`KismetSystemLibrary.PrintString` "Not FAT enough" true true (struct :`G` 0.66 :`B` 1.0 :`A` 1.0) 5.0))))

(fn `UserConstructionScript`)