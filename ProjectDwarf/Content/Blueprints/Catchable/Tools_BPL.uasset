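; Blueprint function library of two small math and movement helpers, kept with the Catchable Blueprints.
; AngleBetweenTwoVectors flattens both vectors to the XY plane and returns their unsigned angle in degrees from the dot product, ignoring height.
; LerpActor places an actor at a point interpolated between two other actors' locations by a given alpha, without sweep or teleport.
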(fn `Angle Between Two Vectors`
  (params (A :type "Vector Structure") (B :type "Vector Structure"))
  (returns (angle :type "Float (double-precision)"))
  ;[1 1 1] Return the angle between two vectors in degrees
  (return (`KismetMathLibrary.Abs` (`KismetMathLibrary.DegAcos` (`KismetMathLibrary.Dot_VectorVector` (`KismetMathLibrary.Normal` (`KismetMathLibrary.MakeVector` A_X A_Y)) (`KismetMathLibrary.Normal` (`KismetMathLibrary.MakeVector` B_X B_Y)))))))

(fn `LerpActor`
  (params (ActorToMove :type "Actor Object Reference") (From :type "Actor Object Reference") (To :type "Actor Object Reference") (lerp :type "Float (double-precision)"))
  (`Actor.K2_SetActorLocation` ActorToMove (`KismetMathLibrary.VLerp` (`Actor.K2_GetActorLocation` From) (`Actor.K2_GetActorLocation` To) lerp) false false))