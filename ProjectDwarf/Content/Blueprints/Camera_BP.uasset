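; Shared two-player camera actor that becomes every player controller's view target and frames both players from GameMode_BP's player list.
; A fast looping timer sets spring arm length from the clamped distance between players and interpolates the actor toward their averaged position.
; The same update calls LimitMoove for player 0, stopping movement when the controller's projected location nears or passes the left or top screen edge.
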(event `self.ReceiveBeginPlay`
  (`self.SpawnPlayers`)
  (`KismetSystemLibrary.K2_SetTimer` null "UpdateCamera" 0.001 true))

(event `UpdateCamera`
  ;[1 1 1] Update Camera Zoom
  (`self.SetArmLengthP2`)
  (`self.SetCameraPosP2`)
  (`self.LimitMoove` 0))

(fn `CalculateDistance`
  (params (`Player ref 1` :type "/Game/Blueprints/Player_BP Object Reference") (`Player ref 2` :type "/Game/Blueprints/Player_BP Object Reference"))
  (returns (Distance :type "Float (double-precision)"))
  (if (and (`KismetSystemLibrary.IsValid` `Player ref 1`) (`KismetSystemLibrary.IsValid` `Player ref 2`))
    (set `self.Distance` (`self.GetDistanceTo` `Player ref 1` `Player ref 2`))
    (else
      (set `self.Distance` 0.0)))
  (return (`self.Distance`)))

(fn `GetLocation`
  (params (Player :type "/Game/Blueprints/Player_BP Object Reference"))
  (returns (Location :type "Vector Structure"))
  (`/Engine/EditorBlueprintResources/StandardMacros.IsValid` Player
    (:`Is Valid`
      (set `self.Location` (`self.K2_GetActorLocation` Player)))
    (:`Is Not Valid`
      (set `self.Location` (0.0 0.0 0.0))))
  (return (`self.Location`)))

(fn `LimitMoove`
  (params (PlayerID :type Integer))
  (bind _returnvalue (`GameplayStatics.GetPlayerController` PlayerID))
  (bind (_screenlocation _returnvalue_2) (`PlayerController.ProjectWorldLocationToScreen` _returnvalue (`self.K2_GetActorLocation` _returnvalue) false))
  (bind (_x _y) (`KismetMathLibrary.BreakVector2D` _screenlocation))
  (if _returnvalue_2
    (if (or (< _x 10.0) (< _y 10.0))
      (`Controller.StopMovement` _returnvalue))))

(fn `SetArmLengthP2`
  (set `SpringArmComponent.TargetArmLength` (`KismetMathLibrary.FClamp` (`self.CalculateDistance` (`self.P1`) (`self.P2`)) (`self.MinArmLength`) (`self.MaxArmLength`)) (`self.SpringArm`)))

(fn `SetCameraPosP2`
  (set `self.TargetPos` (/ (+ (`self.GetLocation` (`self.P1`)) (`self.GetLocation` (`self.P2`))) (`KismetMathLibrary.Conv_IntToDouble` (`KismetArrayLibrary.Array_Length` (`self.PlayersReference`)))))
  (`self.K2_SetActorLocation` (`KismetMathLibrary.VInterpTo` (`self.PreviousPos`) (`self.TargetPos`) (`GameplayStatics.GetWorldDeltaSeconds`) (`self.InterpSpeed`)))
  (set `self.PreviousPos` (`self.K2_GetActorLocation`)))

(fn `SpawnPlayers`
  (bind _camera (`self.Camera`))
  (bind _asgame_mode_bp (cast `/Game/Blueprints/GameMode_BP` (`GameplayStatics.GetGameMode`)))
  (bind _output_get (set `self.GameMode_BP` _asgame_mode_bp))
  (set `self.PlayersReference` (`/Game/Blueprints/GameMode_BP.Players` _output_get))
  (bind _outactors (`GameplayStatics.GetAllActorsOfClass` "/Script/Engine.PlayerController"))
  (`PlayerController.SetViewTargetWithBlend` _outactors self 0.0 "VTBlend_Linear" 0.0 false)
  (for (_array_element _array_index) (`self.PlayersReference`)
    (switch `int` _array_index
      (:`0`
        (bind _output_get_2 (set `self.P1` _array_element))
        (set `/Game/Blueprints/Player_BP.CameraGame` _camera _output_get_2))
      (:`1`
        (bind _output_get_3 (set `self.P2` _array_element))
        (set `/Game/Blueprints/Player_BP.CameraGame` _camera _output_get_3)))))

(fn `UserConstructionScript`)