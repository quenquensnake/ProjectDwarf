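; Campfire actor with a toggleable Fire component and a flickering light, able to signal a switch to night when lit.
; BeginPlay sets Fire visibility from FireActived, then loops forever, randomizing the light intensity after short random delays whether or not the fire is active.
; The ActiveFire event shows the fire and, if SwitchNight is set, calls SwitchNightByCampFire.
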(event `self.ReceiveBeginPlay`
  (if (`self.FireActived`)
    (`SceneComponent.SetVisibility` (`self.Fire`) true false)
    (else
      (`SceneComponent.SetVisibility` (`self.Fire`) false false)))
  ;[1 1 1] Light Flick
  (`LightComponent.SetIntensity` (`self.CampFireLight`) (`KismetMathLibrary.RandomFloatInRange` 15000.0 19000.0) :!label _label)
  (`KismetSystemLibrary.Delay` (`KismetMathLibrary.RandomFloatInRange` 0.0 0.2))
  (goto _label))

(event `ActiveFire`
  (`SceneComponent.SetVisibility` (`self.Fire`) true false)
  (if (`self.SwitchNight`)
    (`self.SwitchNightByCampFire`)))

(fn `UserConstructionScript`)