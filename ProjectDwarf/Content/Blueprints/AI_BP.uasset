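; AI character Blueprint that patrols in a loop through the locations of all TargetPoint actors in the level.
; BeginPlay caches those unique locations in an array, with the actor count as the loop limit.
; Tick issues SimpleMoveToLocation toward the current waypoint; within a fixed radius, it waits on a Delay, prints a debug string, then advances the index, wrapping to zero.
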(event `self.ReceiveBeginPlay`
  ;[0.4179 0 1] IA Waypoints Sytem
  (`self.Init Waypoints`))

(event `self.ReceiveTick`
  (params (DeltaSeconds :type "Float (single-precision)"))
  (bind _output (`|GetArrayItem` (`self.Waypoints`) (`self.IndexWaypoints`)))
  ;[0.4179 0 1] IA Waypoints Sytem
  (`NavigationSystem.SimpleMoveToLocation` (`self.GetController`) _output)
  (if (<= (`KismetMathLibrary.VSize` (- (`self.K2_GetActorLocation`) _output)) 250.0)
    (`KismetSystemLibrary.Delay` 5.0)
    (`KismetSystemLibrary.PrintString` "Hello")
    (`/Engine/EditorBlueprintResources/StandardMacros.IncrementInt` (`self.IndexWaypoints`)
      (:`  `
        (if (>= (`self.IndexWaypoints`) (`self.NumbOfTarget`))
          (set `self.IndexWaypoints` 0))))))

(fn `Init Waypoints`
  ;[0.4179 0 1] Init Waypoints Array
  (bind _outactors (`GameplayStatics.GetAllActorsOfClass` "/Script/Engine.TargetPoint"))
  (bind _output_get (set `self.WaypointsActor` _outactors))
  (for _array_element _output_get
    (`KismetArrayLibrary.Array_AddUnique` (`self.Waypoints`) (`self.K2_GetActorLocation` _array_element)))
  (set `self.NumbOfTarget` (`KismetArrayLibrary.Array_Length` _output_get)))

(fn `UserConstructionScript`)