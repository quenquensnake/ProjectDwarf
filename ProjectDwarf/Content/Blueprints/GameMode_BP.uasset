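; Game mode for a local multiplayer game that shows the title screen on the TitleScreen level, otherwise sets up UI and players.
; Spawns a possessed Player_BP per controller at index-tagged PlayerStarts, giving the second player a dwarf mesh.
; Tick records player locations and copies the camera's distance value.
; Also forwards damage, heal and heart gains to the life widget, and exposes per-sound-class volume setters through a sound mix.
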(event `self.ReceiveBeginPlay`
  (`GameplayStatics.SetBaseSoundMix` "/Game/Sounds/SoundMix.SoundMix")
  (bind _returnvalue (`GameplayStatics.GetCurrentLevelName` true))
  (if (`KismetStringLibrary.EqualEqual_StrStr` _returnvalue "TitleScreen")
    (bind _returnvalue_2 (`|CreateWidget` "/Game/Blueprints/TitleScreen_BP.TitleScreen_BP_C"))
    (`UserWidget.AddToViewport` _returnvalue_2 0)
    (else
      (`self.CreatePlayerUI`)
      (`self.GetPlayerSpawnPoint`)
      (`self.SpawnPlayers`))))

(event `self.ReceiveTick`
  (params (DeltaSeconds :type "Float (single-precision)"))
  (if (> (`KismetArrayLibrary.Array_Length` (`self.Players`)) 0)
    (set `self.DistancePlayers` (`/Game/Blueprints/Camera_BP.Distance` (`self.CameraBP`)))
    (for (_array_element _array_index) (`self.Players`)
      (`KismetArrayLibrary.Array_Set` (`self.Players_Location`) _array_index (`self.K2_GetActorLocation` _array_element)))))

(fn `Change Volume`
  (params (Volume :type "Float (double-precision)"))
  (`GameplayStatics.SetSoundMixClassOverride` "/Game/Sounds/SoundMix.SoundMix" "/Game/Sounds/SC_Master.SC_Master" Volume 1.0 0.0))

(fn `CreatePlayerUI`
  (if (not (`self.IsUIcreated?`))
    (bind _returnvalue (`|CreateWidget` "/Game/UI/Players_Life_BP.Players_Life_BP_C"))
    (bind _output_get (set `self.PlayerLife_BP` _returnvalue))
    (`UserWidget.AddToViewport` _output_get 0)
    (set `self.IsUIcreated?` true)
    (`Widget.SetVisibility` _output_get "Collapsed")
    (bind _returnvalue_2 (`|CreateWidget` "/Game/UI/Warning_Widget.Warning_Widget_C"))
    (`UserWidget.AddToViewport` _returnvalue_2 0)))

(fn `GetPlayerSpawnPoint`
  (bind _outactors (`GameplayStatics.GetAllActorsOfClass` "/Script/Engine.PlayerStart"))
  (set `self.PlayerStartArray` _outactors))

(fn `PlayerAddHeart`
  (params (PlayerID :type Integer))
  (`/Game/UI/Players_Life_BP.AddHeart` (`self.PlayerLife_BP`) PlayerID))

(fn `PlayerDamages`
  (params (PlayerID :type Integer) (Damages :type Integer))
  (`/Game/UI/Players_Life_BP.GetDamagesPlayer` (`self.PlayerLife_BP`) PlayerID Damages))

(fn `PlayerHeal`
  (params (PlayerID :type Integer) (HeartsHealed :type Integer))
  (`/Game/UI/Players_Life_BP.HealPlayer` (`self.PlayerLife_BP`) PlayerID HeartsHealed))

(fn `SpawnPlayers`
  (bind _index (`self.Index`))
  (for _index_2 (range (`self.MaxPlayerCount`))
    (set `self.Index` _index_2)
    (for _array_element (`self.PlayerStartArray`)
      (if (== (`PlayerStart.PlayerStartTag` _array_element) (`KismetStringLibrary.Conv_StringToName` (`KismetStringLibrary.Conv_IntToString` (`self.Index`))))
        (`GameplayStatics.CreatePlayer` (`self.Index`))
        (bind _returnvalue (`|SpawnActorFromClass` "/Game/Blueprints/Player_BP.Player_BP_C" (`self.GetTransform` _array_element) "AlwaysSpawn" "OverrideRootScale"))
        (`Controller.Possess` (`GameplayStatics.GetPlayerController` _index) _returnvalue)
        (`KismetArrayLibrary.Array_AddUnique` (`self.Players`) _returnvalue)
        (set `/Game/Blueprints/Player_BP.Id` _index _returnvalue))))
  (`SkinnedMeshComponent.SetSkinnedAssetAndUpdate` (`Character.Mesh` (`|GetArrayItem` (`self.Players`) 1)) "/Game/Animations/DwarfSkeletalMesh1.DwarfSkeletalMesh1" true))

(fn `UserConstructionScript`)

(fn `Volume Ambiant`
  (params (Volume :type "Float (double-precision)"))
  (`GameplayStatics.SetSoundMixClassOverride` "/Game/Sounds/SoundMix.SoundMix" "/Game/Sounds/SC_Ambiant.SC_Ambiant" Volume 1.0 0.0))

(fn `Volume Music`
  (params (Volume :type "Float (double-precision)"))
  (`GameplayStatics.SetSoundMixClassOverride` "/Game/Sounds/SoundMix.SoundMix" "/Game/Sounds/SC_Music.SC_Music" Volume 1.0 0.0))

(fn `Volume Sound`
  (params (Volume :type "Float (double-precision)"))
  (`GameplayStatics.SetSoundMixClassOverride` "/Game/Sounds/SoundMix.SoundMix" "/Game/Sounds/SC_Sounds.SC_Sounds" Volume 1.0 0.0))