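; Drowning zone actor that sends players who fall into it back to the P1Respawn location, whichever player they are.
; Box overlap flags the drowning animation, disables that player's input, waits a configurable delay, then zeroes linear velocity, applies a Z spin, moves the player and restores input.
; Cube overlap moves the player immediately with no drowning sequence.
; An unconnected per-player respawn loop is left unused.
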(event `self.Cube.OnComponentBeginOverlap`
  (params (OverlappedComponent :type "PrimitiveComponent Object Reference") (OtherActor :type "Actor Object Reference") (OtherComp :type "PrimitiveComponent Object Reference") (OtherBodyIndex :type Integer) (bFromSweep :type Boolean) (SweepResult :type "HitResult Structure (by ref)"))
  (cast `/Game/Blueprints/Player_BP` OtherActor)
  (`self.K2_SetActorRelativeLocation` OtherActor (`self.K2_GetActorLocation` (`self.P1 Respawn`)) false false))

(event `self.Box.OnComponentBeginOverlap`
  (params (OverlappedComponent :type "PrimitiveComponent Object Reference") (OtherActor :type "Actor Object Reference") (OtherComp :type "PrimitiveComponent Object Reference") (OtherBodyIndex :type Integer) (bFromSweep :type Boolean) (SweepResult :type "HitResult Structure (by ref)"))
  (bind _asplayer_bp (cast `/Game/Blueprints/Player_BP` OtherActor))
  (bind _animbp_ref (`/Game/Blueprints/Player_BP.AnimBP_Ref` _asplayer_bp))
  (set `/Game/Animations/DwarfAnimBlueprint.Drowning` true _animbp_ref)
  (bind _returnvalue (`GameplayStatics.GetPlayerController` (`/Game/Blueprints/Player_BP.Id` _asplayer_bp)))
  (`self.DisableInput` _asplayer_bp _returnvalue)
  (`KismetSystemLibrary.Delay` (`self.Seconds_before_drowning`))
  (bind _capsulecomponent (`Character.CapsuleComponent` _asplayer_bp))
  (`PrimitiveComponent.SetAllPhysicsLinearVelocity` _capsulecomponent (0.0 0.0 0.0) false)
  (`PrimitiveComponent.SetAllPhysicsAngularVelocity` _capsulecomponent (`KismetMathLibrary.MakeVector` 0.0 0.0 130.0) false)
  (set `/Game/Animations/DwarfAnimBlueprint.Drowning` false _animbp_ref)
  (`self.K2_SetActorRelativeLocation` OtherActor (`self.K2_GetActorLocation` (`self.P1 Respawn`)) false false)
  (`self.EnableInput` _asplayer_bp _returnvalue))

(fn `UserConstructionScript`)