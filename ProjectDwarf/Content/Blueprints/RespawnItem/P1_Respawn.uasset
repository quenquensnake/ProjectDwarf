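; P1_Respawn is a two-player checkpoint that updates the game mode's respawn location.
; Each Player_BP overlapping the CheckpointSave component sets a flag chosen by its Id, 0 or 1.
; The flags are never cleared here, so the players need not be inside together.
; Once both are set, the checkpoint's root world location becomes GameMode_BP's CurrentCheckpoint, rewritten on every later player overlap.
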(event `self.Checkpoint Save.OnComponentBeginOverlap`
  (params (OverlappedComponent :type "PrimitiveComponent Object Reference") (OtherActor :type "Actor Object Reference") (OtherComp :type "PrimitiveComponent Object Reference") (OtherBodyIndex :type Integer) (bFromSweep :type Boolean) (SweepResult :type "HitResult Structure (by ref)"))
  (bind _asplayer_bp (cast `/Game/Blueprints/Player_BP` OtherActor))
  (`|ExecutionSequence`
    (:`then_0`
      (bind _id (`/Game/Blueprints/Player_BP.Id` _asplayer_bp))
      (if (== _id 0)
        (set `self.Player1 ok` true)
        (elif (== _id 1)
          (set `self.Player2 ok` true))))
    (:`then_1`
      (if (and (`self.Player1 ok`) (`self.Player2 ok`))
        (bind _asgame_mode_bp (cast `/Game/Blueprints/GameMode_BP` (`GameplayStatics.GetGameMode`)))
        (set `/Game/Blueprints/GameMode_BP.CurrentCheckpoint` (`SceneComponent.K2_GetComponentLocation` (`self.DefaultSceneRoot`)) _asgame_mode_bp)))))

(fn `UserConstructionScript`)