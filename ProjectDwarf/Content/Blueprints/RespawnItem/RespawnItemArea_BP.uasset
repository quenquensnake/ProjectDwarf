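; Trigger area that respawns pickup items entering it at spawn points tagged for them.
; When an InteractionPickUpBase_BP overlaps the collider, the area saves it and its respawn enum, then compares saved items against SpawnPoints.
; A match destroys the overlapping item and records that point's transform.
; A second loop spawns the same class at the saved transform, restores its RespawnInfo and removes the processed entries.
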(event `self.Collider.OnComponentBeginOverlap`
  (params (OverlappedComponent :type "PrimitiveComponent Object Reference") (OtherActor :type "Actor Object Reference") (OtherComp :type "PrimitiveComponent Object Reference") (OtherBodyIndex :type Integer) (bFromSweep :type Boolean) (SweepResult :type "HitResult Structure (by ref)"))
  ;[1 1 1] Add items to destruct and respawn
  (bind _asinteraction_pick_up_base_bp (cast `/Game/Blueprints/Interaction/Interactibles/InteractionPickUpBase_BP` OtherActor))
  (`KismetArrayLibrary.Array_AddUnique` (`self.SavedActor`) _asinteraction_pick_up_base_bp)
  (`KismetArrayLibrary.Array_AddUnique` (`self.Infos`) (`/Game/Blueprints/Interaction/Interactibles/InteractionPickUpBase_BP.RespawnInfo` _asinteraction_pick_up_base_bp))
  ;[1 1 1] Compare object enum and respawn enum to repop the object at the good location
  (for _array_element (`self.SpawnPoints`)
    (for _array_element_2 (`self.SavedActor`)
      (if (`|EnumEquality` (`/Game/Blueprints/RespawnItem/RespawnItemPoint.SpawnInfos` _array_element) (`/Game/Blueprints/Interaction/Interactibles/InteractionPickUpBase_BP.RespawnInfo` _array_element_2))
        (`self.K2_DestroyActor` _asinteraction_pick_up_base_bp)
        (`KismetArrayLibrary.Array_AddUnique` (`self.SavedTransform`) (`self.GetTransform` _array_element)))))
  ;[1 1 1] Respawn object and remove it from the saved list
  (for (_array_element_3 _array_index) (`self.SavedActor`)
    (bind _output (`|GetArrayItem` (`self.SavedTransform`) _array_index))
    (bind _returnvalue (`|SpawnActorFromClass` (`GameplayStatics.GetObjectClass` _array_element_3) _output "Undefined" "OverrideRootScale"))
    (`KismetArrayLibrary.Array_RemoveItem` (`self.SavedActor`) _array_element_3)
    (`KismetArrayLibrary.Array_RemoveItem` (`self.SavedTransform`) _output)
    (bind _output_2 (`|GetArrayItem` (`self.Infos`) _array_index))
    (set `/Game/Blueprints/Interaction/Interactibles/InteractionPickUpBase_BP.RespawnInfo` _output_2 _returnvalue)
    (`KismetArrayLibrary.Array_RemoveItem` (`self.Infos`) _output_2)))

(fn `UserConstructionScript`)